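; Spawnable planet or moon actor for the system creator, set up from a data struct with material, radius-based scale and an orbit spline around its central body.
; Moons attach to their parent and transform orbit points into its space.
; Tick detects movement and rebuilds the ring from current distance, snapping the nearest point to the body.
; A helper sphere rescales on a PlayerController view event to ease click-dragging.
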(event Custom|ForceRedraw
  (bind _spline (Variables|Default|GetSpline))
  (bind _sphere (Variables|Default|Getsphere))
  (bind _returnvalue (Transformation|GetWorldLocation _sphere))
  (bind _returnvalue_2 (Class|SplineComponent|FindInputKeyClosesttoWorldLocation _spline _returnvalue))
  (bind _returnvalue_3 (Math|Float|Round _returnvalue_2))
  ;[1 1 1] redraws spline every time the actor moves
  (Utilities|Setcurrentloc (Transformation|GetActorLocation))
  (Spline|ClearSplinePoints (Variables|Default|GetSpline) true)
  (Utilities|SetSplinePoints (Class|GeneralHelpFunctions|GenerateSplineRing (Transformation|GetDistanceTo (Variables|OutsideRefs|Getcentral_body)) 0.0 1.0 12))
  (if (.IsMoon (Utilities|Struct|BreakF_SYST_planet_physics_addition (Variables|Data|GetDataStruct)))
    (for _array_element (Utilities|GetSplinePoints)
      (Spline|AddSplinePoint (Variables|Default|GetSpline) (Math|Transform|TransformLocation (Transformation|GetActorTransform (Variables|OutsideRefs|Getcentral_body)) _array_element) "World" true))
    (else
      ;;[0.9589 0.04957 1] unique draw for planets, as it needs no transforms (sun is 0,0,0)
      (Spline|SetSplinePoints (Variables|Default|GetSpline) (Utilities|GetSplinePoints) "World" true)))
  (Spline|SetLocationatSplinePoint _spline _returnvalue_3 _returnvalue "World" true)
  (Utilities|Array|SetArrayElem (.SplineMap (Utilities|Struct|BreakF_SYST_planet_physics_addition (Variables|Data|GetDataStruct))) _returnvalue_3 (Math|Transform|InverseTransformLocation (Transformation|GetActorTransform (Variables|OutsideRefs|Getcentral_body)) _returnvalue)))

(event Custom|Syst_Plnt_Init
  (params (DataStruct :type F%20SYST%20Planet%20Physics%20Addition%20Structure) (central_star :type Actor%20Object%20Reference))
  (bind _spline_points (Utilities|GetSplinePoints))
  ;[0.7863 0.8467 1] Initialiser
  (Variables|Data|SetDataStruct DataStruct)
  (Variables|OutsideRefs|Setcentral_body central_star)
  (Utilities|FlowControl|Sequence
    (:then_0
      (Rendering|Material|SetMaterial (Variables|Default|Getsphere) 0 (.material (Utilities|Struct|BreakF_SYST_planet_physics_addition (Variables|Data|GetDataStruct))))
      (Transformation|SetWorldScale3D (Variables|Default|Getsphere) (Math|Vector|MakeVector (/ (Math|Conversions|ToFloat(Integer) (.radius (Utilities|Struct|BreakF_SYST_planet_physics_addition (Variables|Data|GetDataStruct)))) 1e+03) (/ (Math|Conversions|ToFloat(Integer) (.radius (Utilities|Struct|BreakF_SYST_planet_physics_addition (Variables|Data|GetDataStruct)))) 1e+03) (/ (Math|Conversions|ToFloat(Integer) (.radius (Utilities|Struct|BreakF_SYST_planet_physics_addition (Variables|Data|GetDataStruct)))) 1e+03)))
      (if (.IsMoon (Utilities|Struct|BreakF_SYST_planet_physics_addition (Variables|Data|GetDataStruct)))
        (Transformation|AttachActorToActor (Variables|OutsideRefs|Getcentral_body) "None" "KeepWorld" "KeepWorld" "KeepWorld" false)))
    (:then_1
      (EventDispatchers|BindEventtoUpdateViewScale (Variables|OutsideRefs|GetPlayerController) (delegate Custom|UpdateVis)))
    (:then_2
      ;;[0.6382 1 0.4972] draws spline
      (if (> (Utilities|Array|Length _spline_points) 0)
        (for _array_element _spline_points
          (Spline|AddSplinePoint (Variables|Default|GetSpline) (Math|Transform|TransformLocation (Transformation|GetActorTransform (Variables|OutsideRefs|Getcentral_body)) _array_element) "World" true))
        (CallFunction|UpdateVis)))))

(event Custom|UpdateVis
  ;[0.7863 0.8467 1] Initialiser
  ;;[1 0 0.05666] dynamically changes the scale the visibility sphere appears to make clicking and dragging easier
  (Transformation|SetWorldScale3D (Variables|Default|Getsee-helper) (+ "4.000000,4.000000,4.000000" (Math|Float|Lerp (/ (Variables|/Game/system_creator/BP_SystemController.BP_SystemController_C|GetPawnLastPos (Variables|OutsideRefs|GetPlayerController)) 1e+03) 3.0 0.5))))

(event EventBeginPlay)

(event Collision|EventActorBeginOverlap
  (params (OtherActor :type Actor%20Object%20Reference)))

(event EventTick
  (params (DeltaSeconds :type Float%20%28single-precision%29))
  (bind _spline (Variables|Default|GetSpline))
  (bind _sphere (Variables|Default|Getsphere))
  (bind _returnvalue (Transformation|GetWorldLocation _sphere))
  (bind _returnvalue_2 (Class|SplineComponent|FindInputKeyClosesttoWorldLocation _spline _returnvalue))
  (bind _returnvalue_3 (Math|Float|Round _returnvalue_2))
  ;[1 1 1] redraws spline every time the actor moves
  (if (Class|KismetMathLibrary|NotEqualExactlyVectorVector (Transformation|GetActorLocation) (.WorldspaceLocation (Utilities|Struct|BreakF_SYST_planet_physics_addition (Variables|Data|GetDataStruct))))
    (Utilities|Setcurrentloc (Transformation|GetActorLocation))
    (Spline|ClearSplinePoints (Variables|Default|GetSpline) true)
    (Utilities|SetSplinePoints (Class|GeneralHelpFunctions|GenerateSplineRing (Transformation|GetDistanceTo (Variables|OutsideRefs|Getcentral_body)) 0.0 1.0 12))
    (if (.IsMoon (Utilities|Struct|BreakF_SYST_planet_physics_addition (Variables|Data|GetDataStruct)))
      (for _array_element (Utilities|GetSplinePoints)
        (Spline|AddSplinePoint (Variables|Default|GetSpline) (Math|Transform|TransformLocation (Transformation|GetActorTransform (Variables|OutsideRefs|Getcentral_body)) _array_element) "World" true))
      (else
        ;;[0.9589 0.04957 1] unique draw for planets, as it needs no transforms (sun is 0,0,0)
        (Spline|SetSplinePoints (Variables|Default|GetSpline) (Utilities|GetSplinePoints) "World" true)))
    (Spline|SetLocationatSplinePoint _spline _returnvalue_3 _returnvalue "World" true)
    (Utilities|Array|SetArrayElem (.SplineMap (Utilities|Struct|BreakF_SYST_planet_physics_addition (Variables|Data|GetDataStruct))) _returnvalue_3 (Math|Transform|InverseTransformLocation (Transformation|GetActorTransform (Variables|OutsideRefs|Getcentral_body)) _returnvalue))))

(fn ConstructionScript
  (Spline|ClearSplinePoints (Variables|Default|GetSpline) true))

(fn GenerateSpline
  (params (orbit_radius :type Float%20%28double-precision%29) (orbit_tilt :type Float%20%28double-precision%29) (orbit_ellipse :type Float%20%28double-precision%29))
  (bind _returnvalue (Class|KismetSystemLibrary|MakeLiteralInteger 6))
  (bind _returnvalue_2 (Class|KismetSystemLibrary|MakeLiteralInteger 2))
  ;[1 0 0] DEPRECATED in favour of a C++ function doing the same, but more light weight
  (Utilities|Array|Clear (Variables|Default|Getspline_points))
  (Variables|Deprecated|Setorbit_radius orbit_radius)
  (Variables|Deprecated|Setorbit_tilt orbit_tilt)
  (Variables|Deprecated|Setorbit_ellipse orbit_ellipse)
  (for _index (range 1 (* _returnvalue _returnvalue_2))
    (Utilities|Array|Add (Variables|Default|Getspline_points) (Math|Vector|MakeVector (* (* (Math|Trig|Sin(Degrees) (* _index (/ (* _returnvalue 10) _returnvalue_2))) (- 2.0 (Variables|Deprecated|Getorbit_ellipse))) (Variables|Deprecated|Getorbit_radius)) (* (Variables|Deprecated|Getorbit_radius) (* (Variables|Deprecated|Getorbit_ellipse) (Math|Trig|Cos(Degrees) (* _index (/ (* _returnvalue 10) _returnvalue_2))))) (* (Variables|Deprecated|Getorbit_radius) (* (Math|Trig|Cos(Degrees) (* _index (/ (* _returnvalue 10) _returnvalue_2))) (Variables|Deprecated|Getorbit_tilt))))))
  (return (Variables|Default|Getspline_points)))

(fn MISNGetParent
  (return 0))

(fn MISNPlanetRadius
  (return (.X (Math|Vector|BreakVector (Transformation|GetWorldScale (Variables|Default|Getsphere))))))