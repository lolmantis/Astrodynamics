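; Spawnable planet or moon actor for the system creator, which draws its orbit as a closed spline around its central body.
; Init stores the body's properties, applies material and scale, sizes the Selected component and attaches moons to their parent.
; When the actor moves, Tick rebuilds the ring from its distance to the central body, offsetting moon points by the parent.
; GenerateSplineRing supplies the points; the Blueprint GenerateSpline is deprecated for a lighter C++ version.
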(event Custom|Init
  (params (name :type Text) (material :type Material%20Instance%20Object%20Reference) (type :type Text) (mass :type Float%20%28double-precision%29) (mass%20relative :type Float%20%28double-precision%29) (radius :type Integer) (radius%20relative :type Float%20%28double-precision%29) (central_star :type Actor%20Object%20Reference) (ismoon :type Boolean))
  (bind _spline_points (Variables|Default|Getspline_points))
  (bind _spline (Variables|Default|GetSpline))
  (Utilities|FlowControl|Sequence
    (:then_0
      (Variables|Default|Setname name))
    (:then_1
      (bind _output_get (Variables|Default|Setmaterial material))
      (Rendering|Material|SetMaterial (Variables|Default|Getsphere) 0 _output_get))
    (:then_2
      (Variables|Default|Settype type))
    (:then_3
      (Variables|Default|Setmass mass))
    (:then_4
      (Variables|Default|Setmass%20relative mass%20relative))
    (:then_5
      (Variables|Default|Setradius radius))
    (:then_6
      (bind _output_get_2 (Variables|Default|Setradius%20relative radius%20relative))
      (Transformation|SetActorScale3D (Components|GetOwner (Variables|Default|Getsphere)) (* _output_get_2 (Transformation|GetActorScale3D))))
    (:then_7
      (Variables|Default|Setcentral_body central_star))
    (:then_8
      (bind _output_get_3 (Variables|Default|Setismoon ismoon))
      (if _output_get_3
        (bind _returnvalue (Transformation|AttachActorToActor (Variables|Default|Getcentral_body) "None" "KeepWorld" "KeepWorld" "KeepWorld" false))
        (Development|PrintString (Utilities|String|ToString(Boolean) _returnvalue))))
    (:then_9
      (Transformation|SetWorldScale3D (Variables|Default|Getselected) (* (Math|Vector|ClampVectorSize (Transformation|GetWorldScale (Variables|Default|Getselected)) 1.0 2e+01) 1.2))
      (Class|LayersBlueprintLibrary|AddActortoLayer self (Variables|Default|GetLayer)))
    (:then_10
      (if (> (Utilities|Array|Length _spline_points) 0)
        (for _array_element _spline_points
          (Spline|AddSplinePoint _spline (Math|Transform|InverseTransformLocation (Math|Transform|MakeTransform (* (.location (Transformation|GetActorTransform (Variables|Default|Getcentral_body))) -1.0) (.rotation (Transformation|GetActorTransform (Variables|Default|Getcentral_body))) (.scale (Transformation|GetActorTransform (Variables|Default|Getcentral_body)))) _array_element) "World" true))
        (Spline|SetClosedLoop _spline true true)))))

(event EventBeginPlay)

(event Collision|EventActorBeginOverlap
  (params (OtherActor :type Actor%20Object%20Reference)))

(event EventTick
  (params (DeltaSeconds :type Float%20%28single-precision%29))
  (bind _returnvalue (Actor|GetAttachParentActor))
  (bind _spline (Variables|Default|GetSpline))
  (bind _spline_2 (Variables|Default|GetSpline))
  (bind _returnvalue_2 (Transformation|GetActorTransform _returnvalue))
  (if (Class|KismetMathLibrary|NotEqualExactlyVectorVector (Transformation|GetActorLocation) (Variables|Default|Getcurrent_location))
    (Variables|Default|Setcurrent_location (Transformation|GetActorLocation))
    (for _index (range 0 (- (Utilities|Array|Length (Variables|Default|Getspline_points)) 1))
      (Spline|RemoveSplinePoint (Variables|Default|GetSpline) _index true))
    (Variables|Default|Setspline_points (Class|GeneralHelpFunctions|GenerateSplineRing (Transformation|GetDistanceTo (Variables|Default|Getcentral_body)) 0.0 1.0 6))
    (if (Variables|Default|Getismoon)
      (for (_array_element _array_index) (Variables|Default|Getspline_points)
        (Utilities|Array|SetArrayElem (Variables|Default|Getspline_points) _array_index (Math|Transform|InverseTransformLocation (Math|Transform|MakeTransform (* (.location _returnvalue_2) -1.0) (.rotation _returnvalue_2) "1.000000,1.000000,1.000000") _array_element)))
      (Spline|SetSplinePoints _spline (Variables|Default|Getspline_points) "World" true)
      (Spline|SetClosedLoop _spline true true)
      (else
        ;[1 1 1] Spline, for moons use local coordinate space
        (Spline|SetSplinePoints _spline_2 (Variables|Default|Getspline_points) "World" true)
        (Spline|SetClosedLoop _spline_2 true true)))))

(fn ConstructionScript)

(fn GenerateSpline
  (params (orbit_radius :type Float%20%28double-precision%29) (orbit_tilt :type Float%20%28double-precision%29) (orbit_ellipse :type Float%20%28double-precision%29))
  (bind _returnvalue (Class|KismetSystemLibrary|MakeLiteralInteger 6))
  (bind _returnvalue_2 (Class|KismetSystemLibrary|MakeLiteralInteger 2))
  ;[1 0 0] DEPRECATED in favour of a C++ function doing the same, but more light weight
  (Utilities|Array|Clear (Variables|Default|Getspline_points))
  (Variables|Default|Setorbit_radius orbit_radius)
  (Variables|Default|Setorbit_tilt orbit_tilt)
  (Variables|Default|Setorbit_ellipse orbit_ellipse)
  (for _index (range 1 (* _returnvalue _returnvalue_2))
    (Utilities|Array|Add (Variables|Default|Getspline_points) (Math|Vector|MakeVector (* (* (Math|Trig|Sin(Degrees) (* _index (/ (* _returnvalue 10) _returnvalue_2))) (- 2.0 (Variables|Default|Getorbit_ellipse))) (Variables|Default|Getorbit_radius)) (* (Variables|Default|Getorbit_radius) (* (Variables|Default|Getorbit_ellipse) (Math|Trig|Cos(Degrees) (* _index (/ (* _returnvalue 10) _returnvalue_2))))) (* (Variables|Default|Getorbit_radius) (* (Math|Trig|Cos(Degrees) (* _index (/ (* _returnvalue 10) _returnvalue_2))) (Variables|Default|Getorbit_tilt))))))
  (return (Variables|Default|Getspline_points)))