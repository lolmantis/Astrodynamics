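; BP_SystemPawn is the pawn for the system creator, providing height-based zoom over a very large scale.
; Mouse wheel input moves the root component along world Z, clamped between a minimum and maximum height.
; Tick is empty and noted as moved to the player controller.
; Leftover right-mouse drag panning, which offsets the actor by scaled viewport mouse deltas, is disconnected and never runs.
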(event EventBeginPlay)

(event Collision|EventActorBeginOverlap
  (params (OtherActor :type Actor%20Object%20Reference)))

(event EventTick
  (params (DeltaSeconds :type Float%20%28single-precision%29))
  ;[1 1 1] moved to player controller
)

(event Input|MouseEvents|MouseWheelAxis
  (params (AxisValue :type Float%20%28single-precision%29))
  (bind _defaultsceneroot (Variables|Default|GetDefaultSceneRoot))
  (bind _returnvalue (Transformation|GetWorldLocation _defaultsceneroot))
  (bind (_x _y _z) (Class|KismetMathLibrary|BreakVector3f _returnvalue))
  (Transformation|SetWorldLocation _defaultsceneroot (Math|Vector|MakeVector _x _y (Math|Float|Clamp(Float) (+ _z (* AxisValue -5e+05)) 8e+05 3e+08)) false false))

(event Input|MouseEvents|MouseWheelUp
  (params (Key :type Key%20Structure :default "None")))

(event Input|MouseEvents|RightMouseButton
  (params (Key :type Key%20Structure :default "None"))
  ;[1 1 1] moved to player controller
)

(event Input|MouseEvents|MouseWheelDown
  (params (Key :type Key%20Structure :default "None")))

(fn ConstructionScript)