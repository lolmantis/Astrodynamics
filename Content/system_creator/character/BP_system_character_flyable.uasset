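; BP_system_character_flyable is a free-flying character for the system creator, steered with mouse look and movement input.
; On BeginPlay it casts its controller to the deprecated system player class and adds the movement Enhanced Input mapping context.
; Look and movement only act while the right mouse button is held, with movement rotated by full control rotation to follow the view in 3D.
; Speed is set but only feeds unused leftover nodes.
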(event Input|EnhancedActionEvents|EnhancedInputActionIA_system_look
  (params (ActionValue :type Vector%202D%20Structure) (ElapsedSeconds :type Float%20%28double-precision%29) (TriggeredSeconds :type Float%20%28double-precision%29) (InputAction :type Input%20Action%20Object%20Reference :default "/Game/system_creator/character/inputs/IA_system_look.IA_system_look"))
  ;[1 1 1] camera
  (:Triggered
    (if (Variables|Default|GetMouseDown)
      (Pawn|Input|AddControllerYawInput (.x ActionValue))
      (bind _result (Math|Float|NegateFloat (.y ActionValue))
        (:%20%20
          (Pawn|Input|AddControllerPitchInput _result))))))

(event Input|EnhancedActionEvents|EnhancedInputActionIA_system_movement
  (params (ActionValue :type Vector :default "0, 0, 0") (ElapsedSeconds :type Float%20%28double-precision%29) (TriggeredSeconds :type Float%20%28double-precision%29) (InputAction :type Input%20Action%20Object%20Reference :default "/Game/system_creator/character/inputs/IA_system_movement.IA_system_movement"))
  (bind _returnvalue (Pawn|GetControlRotation :!class /Script/Engine.Pawn))
  ;[1 1 1] movement
  (:Triggered
    (if (Variables|Default|GetMouseDown)
      (Pawn|Input|AddMovementInput (Math|Vector|RotateVector ActionValue (Math|Rotator|MakeRotator (.roll _returnvalue) (.pitch _returnvalue) (.yaw _returnvalue))) 1.0 true))))

(event EventBeginPlay
  (bind _asbp_system_player (Utilities|Casting|CastToBP_SystemPlayer_DEPRECATED (Pawn|GetController)))
  (Utilities|IsValid (PlayerController|LocalPlayerSubsystems|GetEnhancedInputLocalPlayerSubsystem _asbp_system_player)
    (:Is%20Valid
      (Input|AddMappingContext (PlayerController|LocalPlayerSubsystems|GetEnhancedInputLocalPlayerSubsystem _asbp_system_player) "/Game/system_creator/character/inputs/IM_system_movement_context.IM_system_movement_context" 0 "(bIgnoreAllPressedKeysUntilRelease=True,bForceImmediately=False)")
      (Variables|Default|Setspeed 1e+01))))

(event Input|MouseEvents|RightMouseButton
  (params (Key :type Key%20Structure))
  ;[1 1 1] movement
  (:Pressed
    (Variables|Default|SetMouseDown true))
  (:Released
    (Variables|Default|SetMouseDown false)))

(fn ConstructionScript)