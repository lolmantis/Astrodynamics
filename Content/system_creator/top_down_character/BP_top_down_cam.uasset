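; Top-down camera Blueprint that pans and changes height with the mouse.
; Holding the right mouse button makes Tick convert the viewport cursor delta into a scaled world XY offset of the actor.
; The wheel moves the root along world Z, clamping both the position vector's length and the height.
; That length clamp is measured from the world origin, so it can also shift X and Y.
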(event EventBeginPlay)

(event Collision|EventActorBeginOverlap
  (params (OtherActor :type Actor%20Object%20Reference)))

(event EventTick
  (params (DeltaSeconds :type Float%20%28single-precision%29))
  (if (stale Input|MouseEvents|RightMouseButton _output_get)
    (bind _returnvalue (Class|WidgetLayoutLibrary|GetMousePositiononViewport))
    (Variables|Default|Setnew_m_pos _returnvalue)
    (Transformation|AddActorWorldOffset (Math|Vector|MakeVector (* (.y (- (Variables|Default|Getnew_m_pos) (Variables|Default|Getold_m_pos))) 1e+01) (* (.x (- (Variables|Default|Getnew_m_pos) (Variables|Default|Getold_m_pos))) -1e+01) 0.0))
    (Variables|Default|Setold_m_pos (Variables|Default|Getnew_m_pos))))

(event Input|MouseEvents|MouseWheelAxis
  (params (AxisValue :type Float%20%28single-precision%29))
  (bind _returnvalue (* AxisValue -5e+02))
  (bind _defaultsceneroot (Variables|Default|GetDefaultSceneRoot))
  (bind _returnvalue_2 (Transformation|GetWorldLocation _defaultsceneroot))
  (bind _returnvalue_3 (+ _returnvalue_2 (Math|Vector|MakeVector 0.0 0.0 _returnvalue)))
  (bind _returnvalue_4 (Math|Vector|ClampVectorSize _returnvalue_3 7e+03 5.8e+04))
  (Transformation|SetWorldLocation _defaultsceneroot (Math|Vector|MakeVector (.x _returnvalue_4) (.y _returnvalue_4) (Math|Float|Clamp(Float) (.z _returnvalue_4) 1e+03 5.8e+04)) false false))

(event Input|MouseEvents|RightMouseButton
  (params (Key :type Key%20Structure :default "None"))
  (:Pressed
    (bind _returnvalue (Class|WidgetLayoutLibrary|GetMousePositiononViewport))
    (Variables|Default|Setold_m_pos _returnvalue)
    (bind _output_get (Variables|Default|Setright_mouse true)))
  (:Released
    (Variables|Default|Setright_mouse false)))

(fn ConstructionScript)