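; Top-down player controller for the system creator that drags planets around and spawns new ones near the base star.
; Left click picks the actor under the cursor and opens a Tick gate that moves it by intersecting the mouse ray with its horizontal plane.
; SpawnPlanet reads a DT_PlanetData row and initializes a BP_planet_spawnable, offset from the star by its squared scale.
; Q toggles the pause menu against the main UI.
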(event Custom|SetBaseStar
  (params (BaseStar :type BP%20Default%20Star%20Object%20Reference))
  (Variables|Default|SetBaseStar BaseStar))

(event Custom|setindex
  (params (selected_index :type Integer))
  (Variables|Default|Setselected_index selected_index))

(event EventBeginPlay
  (bind _foundwidgets (Widget|GetAllWidgetsOfClass "/Game/GlobalData/WBP_PauseMenu.WBP_PauseMenu_C" true))
  (if (== (Utilities|Array|Length _foundwidgets) 0)
    (bind _returnvalue (UserInterface|CreateWidget "/Game/GlobalData/WBP_PauseMenu.WBP_PauseMenu_C"))
    (bind _output_get (Variables|Default|SetPauseMenuQuickAccess _returnvalue))
    (UserInterface|Viewport|AddtoViewport _output_get 0)
    (Widget|SetVisibility _output_get "Hidden")
    (Development|ExecuteConsoleCommand "show splines" 0)))

(event EventTick
  (params (DeltaSeconds :type Float%20%28single-precision%29))
  (bind _returnvalue (Game|GetPlayerController 0))
  (bind (_worldlocation _worlddirection) (Game|Player|ConvertMouseLocationToWorldSpace _returnvalue))
  ;[1 1 1] moves planet around world along z plane
  (Utilities|FlowControl|Gate true :!label _label
    (:Exit
      (Utilities|IsValid (stale Input|MouseEvents|LeftMouseButton _output_get)
        (:Is%20Valid
          (Transformation|SetActorLocation (Variables|Default|Getmoved_object) (.Intersection (Class|KismetMathLibrary|LinePlaneIntersectionOriginNormal (Camera|GetCameraLocation (Game|GetPlayerCameraManager 0)) (+ _worldlocation (* _worlddirection 1e+05)) (Transformation|GetActorLocation (Variables|Default|Getmoved_object)) "0.000000,0.000000,1.000000")) false false))
        (:Is%20Not%20Valid
          (goto _label Close))))))

(event Input|MouseEvents|LeftMouseButton
  (params (Key :type Key%20Structure :default "None"))
  (bind _returnvalue (Game|GetPlayerController 0))
  (bind _hitresult (Game|Player|GetHitResultUnderCursorbyChannel _returnvalue "TraceTypeQuery1" true))
  (bind (_worldlocation _worlddirection) (Game|Player|ConvertMouseLocationToWorldSpace _returnvalue))
  (bind (_bblockinghit _binitialoverlap _time _distance _location _impactpoint _normal _impactnormal _physmat _hitactor) (Collision|BreakHitResult _hitresult))
  ;[1 1 1] moves planet around world along z plane
  (:Pressed
    (if _bblockinghit
      (Utilities|IsValid _hitactor
        (:Is%20Valid
          (bind _output_get (Variables|Default|Setmoved_object _hitactor))
          (Utilities|FlowControl|Gate true) ; enters at Open
        ))))
  (:Released
    (Variables|Default|Setmoved_object 0)
    (Utilities|FlowControl|Gate true) ; enters at Close
  ))

(event Input|KeyboardEvents|Q
  (params (Key :type Key%20Structure :default "None"))
  ;[1 1 1] Pause Menu Displayer
  (:Pressed
    (bind _isa (Utilities|FlowControl|FlipFlop)
      (:A
        _)
      (:B
        _))
    (Widget|SetVisibility (Variables|Default|GetPauseMenuQuickAccess) (select _isa "Visible" "Hidden"))
    (Widget|SetVisibility (Variables|Default|GetMainUI) (select _isa "Hidden" "Visible"))))

(event Custom|SpawnPlanet
  (params (DataTableRowName :type Text%20%28by%20ref%29))
  (bind _basestar (Variables|Default|GetBaseStar))
  (bind _sun (Variables|/Game/GlobalData/global_blueprints/BP_DefaultStar.BP_DefaultStar_C|GetSun _basestar))
  (bind _returnvalue (Transformation|GetWorldScale _sun))
  (bind _returnvalue_2 (Transformation|GetWorldTransform _sun))
  (bind _returnvalue_3 (* (.x _returnvalue) (.x _returnvalue)))
  (bind _returnvalue_4 (+ (Math|Vector|MakeVector _returnvalue_3 0.0 0.0) (.location _returnvalue_2)))
  (bind _returnvalue_5 (Math|Transform|MakeTransform _returnvalue_4 (.rotation _returnvalue_2)))
  (bind (_location _rotation) (Math|Transform|BreakTransform _returnvalue_5))
  (bind _returnvalue_6 (Utilities|GetDataTableRow "/Game/planet_creator/DT_PlanetData.DT_PlanetData" (Utilities|String|StringToName (Utilities|String|ToString(Text) DataTableRowName)))
    (:then
      (bind _returnvalue_7 (Game|SpawnActorfromClass "/Game/system_creator/spawned_planet/BP_planet_spawnable.BP_planet_spawnable_C" _returnvalue_5 "Undefined" "MultiplyWithRoot" 0 0))
      (Default|Init _returnvalue_7 (.Planet_name (Utilities|Struct|BreakF_Planet_data _returnvalue_6)) (.Planet_material (Utilities|Struct|BreakF_Planet_data _returnvalue_6)) (.body_type (Utilities|Struct|BreakF_Planet_data _returnvalue_6)) (.Planet_mass (Utilities|Struct|BreakF_Planet_data _returnvalue_6)) (.Earth_rel_mass (Utilities|Struct|BreakF_Planet_data _returnvalue_6)) (.Planet_radius (Utilities|Struct|BreakF_Planet_data _returnvalue_6)) (.Earth_rel_rad (Utilities|Struct|BreakF_Planet_data _returnvalue_6)) (Variables|Default|GetBaseStar) false)
      (Development|PrintText (Utilities|Text|FormatText "{vectorx},{vectory},{vectorz} | {rotationx},{rotationy},{rotationz}" (.x _location) (.y _location) (.z _location) (.roll _rotation) (.pitch _rotation) (.yaw _rotation))))))

(fn ConstructionScript)