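; Player controller for the planet creator, handling mouse manipulation of the Planet and switching between the main UI and pause menu.
; Left-dragging on the planet spins its sphere relative to the spring arm's view, while right-dragging orbits the camera via the spring arm.
; Both drags run on Tick, hiding the cursor and pinning it to its press position.
; Q toggles the pause menu created on BeginPlay, and menu row selections pass to MainUI for loading.
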(event Custom|LMBTick
  (bind (_deltax _deltay) (Class|PlayerController|GetInputMouseDelta))
  (bind _planet (Variables|Default|GetPlanet))
  (bind _returnvalue (* _deltax -1.0))
  (bind _returnvalue_2 (* _deltay -1.0))
  (bind _springarm (Variables|/Game/planet_creator/BP_PLNT_DisplayPlanet.BP_PLNT_DisplayPlanet_C|GetSpringArm _planet))
  (bind _returnvalue_3 (Math|Vector|MakeVector 0.0 _returnvalue _returnvalue_2))
  (bind _returnvalue_4 (Transformation|GetWorldRotation _springarm))
  (bind _returnvalue_5 (Math|Vector|RotateVector _returnvalue_3 (Math|Rotator|MakeRotator 0.0 (.yaw _returnvalue_4) (.pitch _returnvalue_4))))
  ;[1 1 1] Rotates Planet Object
  (if (and (Variables|Default|Getrotate) (Variables|Default|Getleftmousedown))
    ;;[1 0.1812 0.9082] Adjusts rotation by current spring arm camera direction
    (Transformation|AddWorldRotation (Variables|/Game/planet_creator/BP_PLNT_DisplayPlanet.BP_PLNT_DisplayPlanet_C|GetSphere _planet) (Math|Rotator|MakeRotator (.x _returnvalue_5) (.z _returnvalue_5) (.y _returnvalue_5)) false false)
    (Class|PlayerController|SetMouseLocation (Math|Float|Round (Variables|Default|Getmousex)) (Math|Float|Round (Variables|Default|Getmousey)))))

(event Custom|UpdatePlanetFromMenu
  (params (RowName :type Name))
  ;[0.3806 1 0.5073] Quick handover between row table and UI
  (Default|LoadNewfromMenu (Variables|OutsideHandovers|GetMainUI) RowName))

(event Custom|RMBTick
  ;[1 1 1] orbits camera around planet using spring arm
  (if (Variables|Default|Getrightmousedown)
    (Transformation|SetWorldRotation (Variables|/Game/planet_creator/BP_PLNT_DisplayPlanet.BP_PLNT_DisplayPlanet_C|GetSpringArm (Variables|Default|GetPlanet)) (Class|GeneralHelpFunctions|RotateSpringArm self (Variables|/Script/Engine.SceneComponent|GetRelativeRotation (Variables|/Game/planet_creator/BP_PLNT_DisplayPlanet.BP_PLNT_DisplayPlanet_C|GetSpringArm (Variables|Default|GetPlanet)))) false false)
    (Class|PlayerController|SetMouseLocation (Math|Float|Round (Variables|Default|Getmousex)) (Math|Float|Round (Variables|Default|Getmousey)))))

(event EventBeginPlay
  (bind _foundwidgets (Widget|GetAllWidgetsOfClass "/Game/GlobalData/WBP_MAIN_PauseMenu.WBP_MAIN_PauseMenu_C" true))
  (if (== (Utilities|Array|Length _foundwidgets) 0)
    (bind _returnvalue (UserInterface|CreateWidget "/Game/GlobalData/WBP_MAIN_PauseMenu.WBP_MAIN_PauseMenu_C"))
    (bind _output_get (Variables|OutsideHandovers|SetPauseMenuQuickAccess _returnvalue))
    (UserInterface|Viewport|AddtoViewport _output_get 0)
    (Widget|SetVisibility _output_get "Hidden")))

(event EventTick
  (params (DeltaSeconds :type Float%20%28single-precision%29))
  (CallFunction|RMBTick)
  (CallFunction|LMBTick))

(event Input|MouseEvents|LeftMouseButton
  (params (Key :type Key%20Structure))
  (bind (_locationx _locationy) (Game|Player|GetMousePosition))
  ;[1 1 1] Rotates Planet Object
  (:Pressed
    (Variables|Default|Setleftmousedown true)
    (Utilities|FlowControl|Sequence
      (:then_0
        (Variables|Default|Setmousex _locationx)
        (Variables|Default|Setmousey _locationy))
      (:then_1
        (bind _output_get (Variables|Default|Setrotate (== (.HitActor (Collision|BreakHitResult (.HitResult (Game|Player|GetHitResultUnderCursorbyChannel "TraceTypeQuery1" false)))) (Variables|Default|GetPlanet))))
        (if _output_get
          (Variables|Default|SetbShowMouseCursor false)))))
  (:Released
    (Variables|Default|Setleftmousedown false)
    (Variables|Default|SetbShowMouseCursor true)
    (Variables|Default|Setrotate false)))

(event Input|KeyboardEvents|Q
  (params (Key :type Key%20Structure))
  ;[1 1 1] Pause Menu Displayer
  (:Pressed
    (bind _isa (Utilities|FlowControl|FlipFlop)
      (:A
        _)
      (:B
        _))
    (Widget|SetVisibility (Variables|OutsideHandovers|GetPauseMenuQuickAccess) (select _isa "Visible" "Hidden"))
    (Widget|SetVisibility (Variables|OutsideHandovers|GetMainUI) (select _isa "Hidden" "Visible"))))

(event Input|MouseEvents|RightMouseButton
  (params (Key :type Key%20Structure))
  (bind (_locationx _locationy) (Game|Player|GetMousePosition))
  ;[1 1 1] orbits camera around planet using spring arm
  (:Pressed
    (Variables|Default|SetbShowMouseCursor false)
    (Utilities|FlowControl|Sequence
      (:then_0
        (Variables|Default|Setmousex _locationx)
        (Variables|Default|Setmousey _locationy)
        (Variables|Default|Setrightmousedown true))))
  (:Released
    (Variables|Default|SetbShowMouseCursor true)
    (Variables|Default|Setrightmousedown false)))

(fn ConstructionScript)

(fn RotateObjectAroundVector
  (params (Rotating%20Actor :type Vector) (Central%20Actor :type Vector) (Angle :type Float%20%28double-precision%29))
  (LocalVariables|SetRotating%20Actor%20Vector Rotating%20Actor)
  (LocalVariables|SetCenter%20Actor%20Vector Central%20Actor)
  (bind _output_get (LocalVariables|SetOrbit (- (LocalVariables|GetRotating%20Actor%20Vector) (LocalVariables|GetCenter%20Actor%20Vector))))
  (return (- (Math|Vector|RotateVectorAroundAxis _output_get Angle "0.000000,0.000000,1.000000") (LocalVariables|GetOrbit))))