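; Mission creator spacecraft actor that displays a selectable hull: Cassini, New Horizons or OSIRIS-REx.
; UpdateMesh switches on Hull, adding that craft's instanced mesh component and removing the previous instance through a shared helper.
; The construction script seeds a tiny placeholder instance for that swap and removes the first point from the InitialPath and FinalPath splines.
; AddMeshesToSpline bends mesh segments along a given spline into a closed orbit loop.
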(event Custom|UpdateMesh
  (switch name (Variables|Default|Gethull)
    (:HUL_Cassini
      (CallFunction|ISMCassini))
    (:HUL_New_Horizons
      (CallFunction|ISMNewHorizons))
    (:HUL_OSIRIS-REx
      (CallFunction|ISMOSIRIS-REx))))

(event EventBeginPlay)

(event Collision|EventActorBeginOverlap
  (params (OtherActor :type Actor%20Object%20Reference)))

(event EventTick
  (params (DeltaSeconds :type Float%20%28single-precision%29)))

(fn ConstructionScript
  ;[1 1 1] required for instanced mesh comparator to work when adding craft mesh
  (bind _returnvalue (AddComponent|AddInstancedStaticMeshComponent false))
  (Components|InstancedStaticMesh|AddInstance _returnvalue (Math|Transform|MakeTransform "0, 0, 0" "0, 0, 0" "0.001000,0.001000,0.001000") false)
  (Variables|Default|SetInstancedStaticMesh _returnvalue)
  ;[1 1 1] empties spline so circles make sense
  (Spline|RemoveSplinePoint (Variables|Default|GetInitialPath) 0 true)
  (Spline|RemoveSplinePoint (Variables|Default|GetFinalPath) 0 true))

(fn ISMCassini
  (bind _returnvalue (AddComponent|AddInstancedStaticMeshComponent false))
  (bind _output_static_mesh (Utilities|StaticMeshBoilerplate _returnvalue))
  (return _output_static_mesh))

(fn ISMNewHorizons
  (bind _returnvalue (AddComponent|AddInstancedStaticMeshComponent false))
  (bind _output_static_mesh (Utilities|StaticMeshBoilerplate _returnvalue))
  (return _output_static_mesh))

(fn ISMOSIRIS-REx
  (bind _returnvalue (AddComponent|AddInstancedStaticMeshComponent false))
  (bind _output_static_mesh (Utilities|StaticMeshBoilerplate _returnvalue))
  (return _output_static_mesh))

(fn AddMeshestoSpline
  (params (Spline :type Spline%20Component%20Object%20Reference) (Scale :type Vector%202D%20Structure))
  (bind _returnvalue (Spline|GetNumberOfSplinePoints Spline))
  (bind _returnvalue_2 (- _returnvalue 1))
  ;[1 1 1] adds a cylinder mesh I made in blender (it has slices to allow bending) and bends it to make a circle for the path of the planet/moon, still needs tweaking for scales
  (LocalVariables|SetSelectedSpline Spline)
  (for _index (range 0 _returnvalue_2)
    (bind _returnvalue_3 (AddComponent|AddSplineMeshComponent true))
    (SplineMesh|SetStartScale _returnvalue_3 Scale true :!class /Script/Engine.SplineMeshComponent)
    (SplineMesh|SetEndScale _returnvalue_3 Scale true :!class /Script/Engine.SplineMeshComponent)
    (SplineMesh|SetStartandEnd _returnvalue_3 (.Location (Spline|GetLocationandTangentatSplinePoint (LocalVariables|GetSelectedSpline) _index "World")) (.Tangent (Spline|GetLocationandTangentatSplinePoint (LocalVariables|GetSelectedSpline) _index "World")) (.Location (Spline|GetLocationandTangentatSplinePoint (LocalVariables|GetSelectedSpline) (Math|Integer|SelectInt 0 (+ _index 1) (== _index _returnvalue_2)) "World")) (.Tangent (Spline|GetLocationandTangentatSplinePoint (LocalVariables|GetSelectedSpline) (Math|Integer|SelectInt 0 (+ _index 1) (== _index _returnvalue_2)) "World")) true :!class /Script/Engine.SplineMeshComponent))
  (return))