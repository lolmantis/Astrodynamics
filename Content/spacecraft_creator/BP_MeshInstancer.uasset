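; Spacecraft creator actor that swaps the displayed spacecraft model through instanced static mesh components, with options for Cassini, New Horizons and OSIRIS-REx.
; The construction script creates an initial component with one instance and stores it as InstancedMesh.
; Each ISM function adds a new component, uses StaticMeshBoilerplate to remove the previous component's first instance, then adds, stores and returns the new one.
; Previous components are never destroyed, only stripped of that instance.
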(event EventBeginPlay)

(event Collision|EventActorBeginOverlap
  (params (OtherActor :type Actor%20Object%20Reference)))

(event EventTick
  (params (DeltaSeconds :type Float%20%28single-precision%29)))

(fn ConstructionScript
  (bind _returnvalue (AddComponent|AddInstancedStaticMeshComponent false))
  (Components|InstancedStaticMesh|AddInstance _returnvalue (Math|Transform|MakeTransform "0, 0, 0" "0, 0, 0" "1.000000,1.000000,1.000000") false)
  (Variables|Default|SetInstancedMesh _returnvalue))

(fn ISMCassini
  (bind _returnvalue (AddComponent|AddInstancedStaticMeshComponent false))
  (bind _output_static_mesh (Utilities|StaticMeshBoilerplate _returnvalue))
  (Components|InstancedStaticMesh|AddInstance _output_static_mesh (Math|Transform|MakeTransform "0, 0, 0" "0, 0, 0" "1.000000,1.000000,1.000000") false)
  (bind _output_get (Variables|Default|SetInstancedMesh _output_static_mesh))
  (return _output_get))

(fn ISMNewHorizons
  (bind _returnvalue (AddComponent|AddInstancedStaticMeshComponent false))
  (bind _output_static_mesh (Utilities|StaticMeshBoilerplate _returnvalue))
  (Components|InstancedStaticMesh|AddInstance _output_static_mesh (Math|Transform|MakeTransform "0, 0, 0" "0, 0, 0" "1.000000,1.000000,1.000000") false)
  (bind _output_get (Variables|Default|SetInstancedMesh _output_static_mesh))
  (return _output_get))

(fn ISMOSIRISRex
  (bind _returnvalue (AddComponent|AddInstancedStaticMeshComponent false))
  (bind _output_static_mesh (Utilities|StaticMeshBoilerplate _returnvalue))
  (Components|InstancedStaticMesh|AddInstance _output_static_mesh (Math|Transform|MakeTransform "0, 0, 0" "0, 0, 0" "1.000000,1.000000,1.000000") false)
  (bind _output_get (Variables|Default|SetInstancedMesh _output_static_mesh))
  (return _output_get))