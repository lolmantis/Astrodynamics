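; Player controller for the simulator that manages a toggleable pause menu.
; On BeginPlay it creates a hidden pause menu widget in the viewport if no top-level one exists, keeping a reference to it.
; Pressing Q drives a FlipFlop that swaps visibility between the pause menu and MainUI, which is not assigned here.
; The toggle only changes widget visibility and does not pause the game.
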(event EventBeginPlay
  (bind _foundwidgets (Widget|GetAllWidgetsOfClass "/Game/GlobalData/WBP_PauseMenu.WBP_PauseMenu_C" true))
  (if (== (Utilities|Array|Length _foundwidgets) 0)
    (bind _returnvalue (UserInterface|CreateWidget "/Game/GlobalData/WBP_PauseMenu.WBP_PauseMenu_C"))
    (bind _output_get (Variables|Default|SetPauseMenuQuickAccess _returnvalue))
    (UserInterface|Viewport|AddtoViewport _output_get 0)
    (Widget|SetVisibility _output_get "Hidden")))

(event EventTick
  (params (DeltaSeconds :type Float%20%28single-precision%29)))

(event Input|KeyboardEvents|Q
  (params (Key :type Key%20Structure :default "None"))
  ;[1 1 1] Pause Menu Displayer
  (:Pressed
    (bind _isa (Utilities|FlowControl|FlipFlop)
      (:A
        _)
      (:B
        _))
    (Widget|SetVisibility (Variables|Default|GetPauseMenuQuickAccess) (select _isa "Visible" "Hidden"))
    (Widget|SetVisibility (Variables|Default|GetMainUI) (select _isa "Hidden" "Visible"))))

(fn ConstructionScript)