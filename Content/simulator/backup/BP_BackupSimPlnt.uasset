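; Simulated planet or moon actor for a solar system simulator, apparently a backup with orbital motion disconnected.
; Setup stores the body data, applies its texture and attaches it to the default star or a moon's parent planet.
; A spline builds the visible orbit from spline meshes, but Tick is empty and initial velocity returns zero.
; A timer drives mouse camera orbiting, while scroll zoom switches between arm length outward and FOV inward.
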(event Custom|SetTickRate
  (params (Tickrate :type Float%20%28double-precision%29))
  (CallFunction|SIMSetActorTickRate Tickrate))

(event Custom|__BeginPlay
  ;[1 1 1] I've only chained the events HERE because this function becomes too large to justify keeping it next to its binding when it needs so much space
  (Utilities|IsValid (Variables|References|GetSIMController)
    (:Is%20Valid
      (Development|PrintString "Play Request recieved")
      (Utilities|FlowControl|DoOnce false
        (:Completed
          (Default|CallInitVelGenerated (Variables|Astrophysics|GetStartVel))
          (Actor|Tick|SetActorTickEnabled true))))))

(event Custom|GenerateInitialVelocity
  ;[1 1 1] carefully now, this needs to have EVERYTHING instanced beforehand, spline included
  (bind _forcevector (CallFunction|InitialVel))
  (Variables|Astrophysics|SetOrbitVelocity%20in%20km/s (Math|Vector|VectorLength _forcevector))
  (Variables|Default|SetOrbitProgress (Class|SplineComponent|GetDistanceAlongSplineatSplineInputKey (Variables|Default|GetOrbitPath) (Class|SplineComponent|FindInputKeyClosesttoWorldLocation (Variables|Default|GetOrbitPath) (Transformation|GetWorldLocation (Variables|Default|GetSphereMesh))))))

(event Custom|EndPlay
  (Actor|DestroyActor))

(event Custom|AssignOrbitCenter
  (params (Default%20Star :type BP%20Default%20Star%20Object%20Reference) (Sim%20Planets :type Array%20of%20BP%20Sim%20Planet%20Object%20References))
  (bind _data (Variables|Default|GetData))
  (bind (_name _bodytype _surfacetexture _mass _erelmass _radius _erelradius _worldpos _splinemap _centralstar _bismoon) (Utilities|Struct|BreakLoadedValuesStruct _data))
  (bind _output (Utilities|Array|Get(acopy) Sim%20Planets _centralstar))
  (if _bismoon
    (Variables|Default|SetParentBody _output)
    (Transformation|AttachComponentToComponent (Variables|/Script/Astrodynamics_Actual.physics_applicable_planet_base|GetSphereMesh _output) "None" "KeepWorld" "KeepWorld" "KeepWorld" false)
    (else
      (bind _output_get (Variables|Default|SetParentBody Default%20Star))
      (Transformation|AttachActorToActor _output_get "None" "KeepWorld" "KeepWorld" "KeepWorld" false))))

(event Custom|InitBinds
  (bind _simcontroller (Variables|References|GetSIMController))
  (Utilities|IsValid _simcontroller
    (:Is%20Valid
      (EventDispatchers|BindEventtoBroadcastBeginPlay _simcontroller (delegate Custom|BeginPlay))
      (EventDispatchers|BindEventtoBroadcastTickRate _simcontroller (delegate Custom|SetTickRate))
      (EventDispatchers|BindEventtoBroadcastEndPlay _simcontroller (delegate Custom|EndPlay)))))

(event Custom|BeginPlay
  (CallFunction|BeginPlay))

(event EventMISNRotateActor
  ;[1 1 1] quick handover but gets the job done
  (CallFunction|Rotate))

(event EventTick
  (params (DeltaSeconds :type Float%20%28single-precision%29))
  ;[1 1 1] ol' reliable, just moves the planet along its set track, needs to have the spline do the compensating for any gravity occurences though
)

(event EventBeginPlay)

(event BroadcastTickRate(SIMController)
  (params (Tickrate :type Float%20%28double-precision%29))
  (Utilities|IsValid (Variables|References|GetSIMController)
    (:Is%20Valid
      (CallFunction|SIMSetActorTickRate Tickrate))))

(event Custom|Rotate
  (Transformation|SetRelativeRotation (Variables|Default|GetCameraArm) (Class|GeneralHelpFunctions|RotateSpringArm (Game|GetPlayerController 0) (Variables|/Script/Engine.SceneComponent|GetRelativeRotation (Variables|Default|GetCameraArm))) false false)
  (Class|MissionPlayerController|SnapMousetoCenter (Game|GetPlayerController 0)))

(event EventSIMScrollWheel
  (params (AxisValue :type Float%20%28double-precision%29))
  (bind _initspringlength (Variables|Default|GetInitSpringLength))
  (bind _camera (Variables|Default|GetCamera))
  (bind _fieldofview (Variables|/Script/Engine.CameraComponent|GetFieldOfView _camera))
  (bind _returnvalue (== 1e+02 _fieldofview))
  (if (!= AxisValue 0.0)
    (if (and (== (Variables|/Script/Engine.SpringArmComponent|GetTargetArmLength (Variables|Default|GetCameraArm)) (Variables|Default|GetInitSpringLength)) _returnvalue)
      (if (> 0.0 AxisValue)
        (Variables|/Script/Engine.SpringArmComponent|SetTargetArmLength (Variables|Default|GetCameraArm) (Math|Float|Clamp(Float) (+ (Variables|/Script/Engine.SpringArmComponent|GetTargetArmLength (Variables|Default|GetCameraArm)) (* (* AxisValue -1.0) (/ (* (Variables|Default|GetInitSpringLength) 3.0) 1e+02))) _initspringlength (* _initspringlength 3.0)) :!label _label)
        (else
          (Camera|SetFieldOfView (Variables|Default|GetCamera) (Math|Float|Clamp(Float) (+ (* AxisValue -1.0) (Variables|/Script/Engine.CameraComponent|GetFieldOfView (Variables|Default|GetCamera))) 1e+01 1e+02) :!label _label_2)))
      (elif _returnvalue
        (goto _label)
        (else
          (goto _label_2))))))

(fn ConstructionScript
  (Spline|RemoveSplinePoint (Variables|Default|GetSpacecraftDraw) 0 true))

(fn MessySetupNeatened
  (params (Data :type Loaded%20Values%20Struct%20Structure) (Default%20Star :type BP%20Default%20Star%20Object%20Reference) (Sim%20Planets :type Array%20of%20BP%20Sim%20Planet%20Object%20References) (Surface%20Texture :type Material%20Instance%20Object%20Reference) (PlayerController :type BP%20SIM%20Controller%20Object%20Reference))
  (Utilities|FlowControl|Sequence
    (:then_0
      (Utilities|IsValid PlayerController
        (:Is%20Valid
          (Variables|References|SetSIMController PlayerController))))
    (:then_1
      (Variables|Default|SetData Data)
      (CallFunction|AssignOrbitCenter Default%20Star Sim%20Planets)
      (Class|PhysicsApplicablePlanetBase|SetMaterial Surface%20Texture))))

(fn AddSplineMeshes
  (bind _orbitpath (Variables|Default|GetOrbitPath))
  (bind _returnvalue (Spline|GetNumberOfSplinePoints _orbitpath))
  (bind _returnvalue_2 (- _returnvalue 1))
  ;[1 1 1] adds a cylinder mesh I made in blender (it has slices to allow bending) and bends it to make a circle for the path of the planet/moon
  (for _index (range 0 _returnvalue_2)
    (bind _returnvalue_3 (AddComponent|AddSplineMeshComponent true))
    (SplineMesh|SetStartScale _returnvalue_3 "(X=400.000000,Y=400.000000)" true :!class /Script/Engine.SplineMeshComponent)
    (SplineMesh|SetEndScale _returnvalue_3 "(X=400.000000,Y=400.000000)" true :!class /Script/Engine.SplineMeshComponent)
    (SplineMesh|SetStartandEnd _returnvalue_3 (.Location (Spline|GetLocationandTangentatSplinePoint (Variables|Default|GetOrbitPath) _index "World")) (.Tangent (Spline|GetLocationandTangentatSplinePoint (Variables|Default|GetOrbitPath) _index "World")) (.Location (Spline|GetLocationandTangentatSplinePoint (Variables|Default|GetOrbitPath) (Math|Integer|SelectInt 0 (+ _index 1) (== _index _returnvalue_2)) "World")) (.Tangent (Spline|GetLocationandTangentatSplinePoint (Variables|Default|GetOrbitPath) (Math|Integer|SelectInt 0 (+ _index 1) (== _index _returnvalue_2)) "World")) true :!class /Script/Engine.SplineMeshComponent))
  (return))

(fn InitialVel
  ;[1 1 1] for some reason Earth at 1AU has an orbital velocity of 941 km/s and a period of 0.11 days, we've done the math by hand and it should be 40 km/s, figure this shit out quickly
  (Development|PrintString (Utilities|String|ToString(Float) (.Mass (Utilities|Struct|BreakLoadedValuesStruct (Variables|/Script/Astrodynamics_Actual.physics_applicable_planet_base|GetData (Variables|Default|GetParentBody))))))
  (Development|PrintString (Utilities|String|ToString(Float) (Math|Vector|VectorLength "0, 0, 0")))
  (return "0, 0, 0"))

(fn MISNGetParent
  (return 0))

(fn MISNPlanetRadius)

(fn SIMGetOrbitLoc
  (return (Transformation|GetWorldLocation (Variables|Default|GetSphereMesh))))

(fn SIMOrbitCamera
  (params (Enabled? :type Boolean))
  (if Enabled?
    (Utilities|Time|SetTimerbyFunctionName 0 "Rotate" 0.01 true)
    (else
      (Utilities|Time|ClearTimerbyFunctionName 0 "Rotate")))
  (return))

(fn SIMSetActorDoTick
  (params (InDoTick :type Boolean))
  (return))

(fn SIMSetActorTickRate
  (params (NewTickRate :type Float%20%28double-precision%29))
  (Actor|Tick|SetActorTickInterval NewTickRate)
  (return))