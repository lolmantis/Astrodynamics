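; Simulated spacecraft actor, apparently a base for craft, that moves among planets in a space simulator.
; On the controller's begin-play broadcast it applies a one-time orbital impulse around its start planet, then enables Tick to run semi-implicit Euler integration over all planets.
; Controller broadcasts also set its tick interval.
; A timer-driven orbit camera rotates the spring arm, while scrolling switches between arm length and FOV zoom.
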(event Custom|Temp
  ;[1 1 1] temporary just for easier viewing
  (Spline|ClearSplinePoints (Variables|Default|GetFinalPath) true)
  (Spline|ClearSplinePoints (Variables|Default|GetInitialPath) true))

(event Custom|BeginPlayReciever
  ;[1 1 1] begins play, but only once as a safety check to prevent double clicks
  (Utilities|FlowControl|DoOnce false
    (:Completed
      (CallFunction|InitialVelocity)
      (Actor|Tick|SetActorTickEnabled true))))

(event Custom|TickReciever
  ;[1 1 1] globally updates tick with an event dispatch
  (CallFunction|SIMSetActorTickRate (Variables|/Game/simulator/BP_SIM_Controller.BP_SIM_Controller_C|Getsystem%20tick%20rate (Variables|Default|GetSIMController))))

(event Custom|Initialise%20Bindings
  (EventDispatchers|BindEventtoBroadcastTickRate (Variables|Default|GetSIMController) (delegate Custom|TickReciever))
  (EventDispatchers|BindEventtoBroadcastBeginPlay (Variables|Default|GetSIMController) (delegate Custom|BeginPlayReciever)))

(event EventBeginPlay
  (Variables|Default|SetMinSpringArmLength (Variables|/Script/Engine.SpringArmComponent|GetTargetArmLength (Variables|Default|GetCameraArm))))

(event Collision|EventActorBeginOverlap
  (params (OtherActor :type Actor%20Object%20Reference))
  (|CallParentFunction OtherActor) ; This node is disabled and will not be called.\nDrag off pins to build functionality.
)

(event EventTick
  (params (DeltaSeconds :type Float%20%28single-precision%29))
  (Class|Spacecraft|SemiImplicitEuler DeltaSeconds self (Variables|Default|GetPlanets))
  (Variables|Default|SetVelocity (Transformation|GetVelocity)))

(event EventSIMScrollWheel
  (params (AxisValue :type Float%20%28double-precision%29))
  (bind _minspringarmlength (Variables|Default|GetMinSpringArmLength))
  (bind _camera (Variables|Default|GetCamera))
  (bind _fieldofview (Variables|/Script/Engine.CameraComponent|GetFieldOfView _camera))
  (bind _returnvalue (== 45.0 _fieldofview))
  (if (!= AxisValue 0.0)
    (if (and (== (Variables|/Script/Engine.SpringArmComponent|GetTargetArmLength (Variables|Default|GetCameraArm)) (Variables|Default|GetMinSpringArmLength)) _returnvalue)
      (if (> 0.0 AxisValue)
        (Variables|/Script/Engine.SpringArmComponent|SetTargetArmLength (Variables|Default|GetCameraArm) (Math|Float|Clamp(Float) (+ (Variables|/Script/Engine.SpringArmComponent|GetTargetArmLength (Variables|Default|GetCameraArm)) (* (* AxisValue -1.0) (/ (* (Variables|Default|GetMinSpringArmLength) 3.0) 1e+02))) _minspringarmlength (* _minspringarmlength 3.0)) :!label _label)
        (else
          (Camera|SetFieldOfView (Variables|Default|GetCamera) (Math|Float|Clamp(Float) (+ (* AxisValue -1.0) (Variables|/Script/Engine.CameraComponent|GetFieldOfView (Variables|Default|GetCamera))) 6.0 45.0) :!label _label_2)))
      (elif _returnvalue
        (goto _label)
        (else
          (goto _label_2))))))

(event Custom|Rotate
  (Transformation|SetRelativeRotation (Variables|Default|GetCameraArm) (Class|GeneralHelpFunctions|RotateSpringArm (Variables|Default|GetSIMController) (Variables|/Script/Engine.SceneComponent|GetRelativeRotation (Variables|Default|GetCameraArm))) false false)
  (Class|MissionPlayerController|SnapMousetoCenter (Variables|Default|GetSIMController)))

(fn ConstructionScript
  (|CallParentFunction)
  (Physics|SetSimulatePhysics (Variables|Default|GetInstancedStaticMesh) true)
  (Class|PrimitiveComponent|SetMassOverrideinKg (Variables|Default|GetSphere) "None" 1.0 true))

(fn InitialVelocity
  (bind _returnvalue (Transformation|GetActorLocation))
  (bind _startplanetorbit (Variables|Default|GetStartPlanetOrbit))
  (bind _planets (Variables|Default|GetPlanets))
  (bind _output (Utilities|Array|Get(acopy) _planets _startplanetorbit))
  (bind _returnvalue_2 (Transformation|GetActorLocation _output))
  (bind _returnvalue_3 (- _returnvalue _returnvalue_2))
  ;[1 1 1] THIS WORKS
  (Physics|AddImpulse (Variables|Default|GetSphere) (Class|Spacecraft|OrbitInitialForce _returnvalue_3 (Math|Vector|CrossProduct _returnvalue_3 "0.000000,0.000000,1.000000") (.Mass (Utilities|Struct|BreakLoadedValuesStruct (Variables|/Script/Astrodynamics_Actual.physics_applicable_planet_base|GetData _output)))) "None" false))

(fn SIMOrbitCamera
  (params (Enabled? :type Boolean))
  (if Enabled?
    (Utilities|Time|SetTimerbyFunctionName 0 "Rotate" 0.01 true)
    (else
      (Utilities|Time|ClearTimerbyFunctionName 0 "Rotate")))
  (return))

(fn SIMSetActorDoTick
  (params (InDoTick :type Boolean))
  (return))

(fn SIMSetActorTickRate
  (params (NewTickRate :type Float%20%28double-precision%29))
  (Actor|Tick|SetActorTickInterval NewTickRate)
  (return))