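; Simulated planet or moon actor for an orbital simulator, configured from data with mass, scale, tilt, material and parent body.
; Start velocity follows the orbit spline's tangent, is applied as an impulse on play, and cascades to moons to preserve relative motion.
; Tick runs semi-implicit Euler over the controller's physics planets, replacing deprecated spline movement.
; Controller dispatchers drive play, tick rate, teardown and direction arrow; an orbit camera zooms by arm length or FOV.
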(event OnComponentHit(SphereMesh)
  (params (HitComponent :type Primitive%20Component%20Object%20Reference) (OtherActor :type Actor%20Object%20Reference) (OtherComp :type Primitive%20Component%20Object%20Reference) (NormalImpulse :type Vector :default "0, 0, 0") (Hit :type Hit%20Result%20Structure%20%28by%20ref%29))
  (Development|PrintString "Oh Fuck!"))

(event Custom|__BeginDemo
  ;[1 1 1] I've only chained the events HERE because this function becomes too large to justify keeping it next to its binding when it needs so much space
  (Utilities|IsValid (Variables|References|GetSIMController)
    (:Is%20Valid
      (Development|PrintString "Play Request recieved")
      (Utilities|FlowControl|DoOnce false
        (:Completed
          (Physics|AddImpulse (Variables|Default|GetPlanetRoot) (Variables|Astrophysics|GetRelativeStartVel) "None" true)
          (CallFunction|ParentPlanetTranslation "0, 0, 0")
          (Actor|Tick|SetActorTickEnabled true)
          (Variables|/Script/Engine.RotatingMovementComponent|SetRotationRate (Variables|Default|GetRotatingMovement) (* (Variables|Default|GetInitialPeriodVel) (/ (Math|Trig|GetPI) 1.8e+02))))))))

(event Custom|PostSetupEventCall
  (bind _parentbody (Variables|Default|GetParentBody))
  (bind _data (Variables|/Script/Astrodynamics_Actual.physics_applicable_planet_base|GetData _parentbody))
  (bind (_name _bodytype _surfacetexture _mass) (Utilities|Struct|BreakLoadedValuesStruct _data))
  ;[1 1 1] carefully now, this needs to have EVERYTHING instanced beforehand, spline included -- called on system load in control
  (bind _forcevector (CallFunction|InitialVel))
  (Variables|Astrophysics|SetOrbitVelocity%20in%20m/s (Math|Vector|VectorLength _forcevector))
  (Variables|Default|SetOrbitProgress (Class|SplineComponent|GetDistanceAlongSplineatSplineInputKey (Utilities|SIMOrbitPath) (Class|SplineComponent|FindInputKeyClosesttoWorldLocation (Utilities|SIMOrbitPath) (Transformation|GetWorldLocation (Variables|Default|GetSphereMesh)))))
  (Variables|Default|SetPeriodYears (Class|GeneralHelpFunctions|KeplerThirdLaw (Transformation|GetDistanceTo _parentbody) _mass (.Mass (Utilities|Struct|BreakLoadedValuesStruct (Variables|Default|GetData))) (Utilities|Enum|Equal(Enum) _name (Utilities|Text|MakeLiteralText "Sun"))))
  (bind _returnvalue (Class|PhysicsApplicablePlanetBase|GetAngularRotation (.Period (Utilities|Struct|BreakLoadedValuesStruct (Variables|Default|GetData)))))
  (bind _output_get (Variables|Default|SetInitialPeriodVel _returnvalue))
  (Development|PrintString (Utilities|String|ToString(Rotator) _output_get) true true "(R=1.000000,G=0.271898,B=0.000000,A=1.000000)" 6.0))

(event Custom|AssignOrbitCenter
  (params (Default%20Star :type BP%20Default%20Star%20Object%20Reference) (Sim%20Planets :type Array%20of%20BP%20Sim%20Planet%20Object%20References))
  (bind _data (Variables|Default|GetData))
  (bind (_name _bodytype _surfacetexture _mass _period _radius _tilt _worldpos _splinemap _centralstar _bismoon) (Utilities|Struct|BreakLoadedValuesStruct _data))
  (if _bismoon
    (bind _output_get (Variables|Default|SetParentBody (Utilities|Array|Get(acopy) Sim%20Planets _centralstar)))
    (Utilities|Array|Add (Variables|/Script/Astrodynamics_Actual.physics_applicable_planet_base|GetMoons _output_get) self)
    (else
      (Variables|Default|SetParentBody Default%20Star))))

(event EventMISNRotateActor
  ;[1 1 1] quick handover but gets the job done
  (CallFunction|RotateCam))

(event EventEndPlay
  (params (EndPlayReason :type EEndPlayReason%20Enum :default "Destroyed"))
  (Development|PrintString (Utilities|String|Append (Utilities|String|ToString(Text) (.Name (Utilities|Struct|BreakLoadedValuesStruct (Variables|Default|GetData)))) " ended play on reason: " (Utilities|String|EnumtoString EndPlayReason))))

(event EventTick
  (params (DeltaSeconds :type Float%20%28single-precision%29))
  (Class|PhysicsApplicablePlanetBase|SemiImplicitEuler DeltaSeconds (Variables|/Game/simulator/BP_SIM_Controller.BP_SIM_Controller_C|GetPhysicsPlanets (Variables|References|GetSIMController)))
  (Variables|Default|SetDynamicVel (Class|PhysicsApplicablePlanetBase|GetPlanetWorldVel))
  (if (Variables|Default|GetShowDirection)
    (Transformation|SetWorldRotation (Variables|Default|GetForceDirectionArm) (Math|Conversions|RotationFromXVector (- (Class|PhysicsApplicablePlanetBase|GetPlanetWorldVel (Variables|Default|GetParentBody)) (Variables|Default|GetDynamicVel))) false false)))

(event EventChangeHighlightColour
  (params (Color :type Vector :default "0, 0, 0"))
  (Rendering|Material|SetVectorParameterValueonMaterials (Variables|Default|GetVisibility) "Color" Color))

(event EventBeginPlay
  (Components|Movement|SetUpdatedComponent (Variables|Default|GetRotatingMovement) (Variables|Default|GetSphereMesh)))

(event OnClicked(SphereMesh)
  (params (TouchedComponent :type Primitive%20Component%20Object%20Reference) (ButtonPressed :type Key%20Structure :default "None"))
  (Development|PrintString "Planet Clicked"))

(event BroadcastTickRate(SIMController)
  (params (Tickrate :type Float%20%28double-precision%29))
  (Utilities|IsValid (Variables|References|GetSIMController)
    (:Is%20Valid
      (CallFunction|SIMSetActorTickRate Tickrate))))

(event Custom|Listen%20SetTickRate
  (params (Tickrate :type Float%20%28double-precision%29))
  (CallFunction|SIMSetActorTickRate Tickrate))

(event Custom|RotateCam
  (Transformation|SetRelativeRotation (Variables|Default|GetCameraArm) (Class|GeneralHelpFunctions|RotateSpringArm (Game|GetPlayerController 0) (Variables|/Script/Engine.SceneComponent|GetRelativeRotation (Variables|Default|GetCameraArm))) false false)
  (Class|MissionPlayerController|SnapMousetoCenter (Game|GetPlayerController 0)))

(event Custom|ParentPlanetTranslation
  (params (Velocity :type Vector))
  ;[1 1 1] hands down parent velocity to children to maintain relative velocities
  (Utilities|FlowControl|DoOnce false
    (:Completed
      (bind _output_get (Variables|Astrophysics|SetWorldStartVel Velocity))
      (Physics|AddImpulse (Variables|Default|GetPlanetRoot) _output_get "None" true)
      (Default|CallInitVelGeneratedSpacecraft (+ _output_get (Variables|Astrophysics|GetRelativeStartVel)))
      (for _array_element (Variables|Default|GetMoons)
        (Physics|AddImpulse (Variables|/Script/Astrodynamics_Actual.physics_applicable_planet_base|GetPlanetRoot _array_element) (Variables|Astrophysics|GetWorldStartVel) "None" true)
        (bind _asbp_sim_planet (Utilities|Casting|CastToBP_sim_planet _array_element))
        (Default|CallInitVelGenerated _asbp_sim_planet (+ (Variables|Astrophysics|GetWorldStartVel) (Variables|Astrophysics|GetRelativeStartVel)))))))

(event Custom|Listen%20EndPlay
  (Actor|DestroyActor))

(event Custom|Listen%20Show%20Direction
  (params (Yes/No :type Boolean))
  (bind _output_get (Variables|Default|SetShowDirection Yes/No))
  (Rendering|SetVisibility (Variables|Default|GetDirection) _output_get false))

(event Custom|InitBinds
  (bind _simcontroller (Variables|References|GetSIMController))
  (Utilities|IsValid _simcontroller
    (:Is%20Valid
      (EventDispatchers|BindEventtoBroadcastBeginPlay _simcontroller (delegate Custom|Listen%20BeginPlay))
      (EventDispatchers|BindEventtoBroadcastTickRate _simcontroller (delegate Custom|Listen%20SetTickRate))
      (EventDispatchers|BindEventtoBroadcastEndPlay _simcontroller (delegate Custom|Listen%20EndPlay))
      (EventDispatchers|BindEventtoInitVelGenerated (delegate Custom|ParentPlanetTranslation))
      (EventDispatchers|BindEventtoBroadcastShowDirection (Variables|References|GetSIMController) (delegate Custom|Listen%20Show%20Direction)))))

(event Custom|Listen%20BeginPlay
  (CallFunction|BeginDemo))

(event EventSIMScrollWheel
  (params (AxisValue :type Float%20%28double-precision%29))
  (bind _initspringlength (Variables|Default|GetInitSpringLength))
  (bind _camera (Variables|Default|GetCamera))
  (bind _fieldofview (Variables|/Script/Engine.CameraComponent|GetFieldOfView _camera))
  (bind _returnvalue (== 1e+02 _fieldofview))
  (if (!= AxisValue 0.0)
    (if (and (== (Variables|/Script/Engine.SpringArmComponent|GetTargetArmLength (Variables|Default|GetCameraArm)) (Variables|Default|GetInitSpringLength)) _returnvalue)
      (if (> 0.0 AxisValue)
        (Variables|/Script/Engine.SpringArmComponent|SetTargetArmLength (Variables|Default|GetCameraArm) (Math|Float|Clamp(Float) (+ (Variables|/Script/Engine.SpringArmComponent|GetTargetArmLength (Variables|Default|GetCameraArm)) (* (* AxisValue -1.0) (/ (* (Variables|Default|GetInitSpringLength) 3.0) 1e+02))) _initspringlength (* _initspringlength 3.0)) :!label _label)
        (else
          (Camera|SetFieldOfView (Variables|Default|GetCamera) (Math|Float|Clamp(Float) (+ (* AxisValue -1.0) (Variables|/Script/Engine.CameraComponent|GetFieldOfView (Variables|Default|GetCamera))) 1e+01 1e+02) :!label _label_2)))
      (elif _returnvalue
        (goto _label)
        (else
          (goto _label_2))))))

(fn ConstructionScript
  (Spline|RemoveSplinePoint (Variables|Default|GetSpacecraftDraw) 0 true))

(fn MessySetupNeatened
  (params (Data :type Loaded%20Values%20Struct%20Structure) (Default%20Star :type BP%20Default%20Star%20Object%20Reference) (Sim%20Planets :type Array%20of%20BP%20Sim%20Planet%20Object%20References) (Surface%20Texture :type Material%20Instance%20Object%20Reference) (PlayerController :type BP%20SIM%20Controller%20Object%20Reference))
  (Utilities|FlowControl|Sequence
    (:then_0
      (Utilities|IsValid PlayerController
        (:Is%20Valid
          (Variables|References|SetSIMController PlayerController))))
    (:then_1
      (Variables|Default|SetData Data)
      (CallFunction|AssignOrbitCenter Default%20Star Sim%20Planets)
      (Class|PhysicsApplicablePlanetBase|SetMaterial Surface%20Texture)
      ;[1 1 1] update scale
      (Transformation|SetWorldScale3D (Variables|Default|GetSphereMesh) (Math|Vector|MakeVector (Math|Conversions|ToFloat(Integer) (* (.Radius (Utilities|Struct|BreakLoadedValuesStruct (Variables|Default|GetData))) 1000)) (Math|Conversions|ToFloat(Integer) (* (.Radius (Utilities|Struct|BreakLoadedValuesStruct (Variables|Default|GetData))) 1000)) (Math|Conversions|ToFloat(Integer) (* (.Radius (Utilities|Struct|BreakLoadedValuesStruct (Variables|Default|GetData))) 1000))))
      (bind _output_get (Variables|/Script/Engine.SpringArmComponent|SetTargetArmLength (Variables|Default|GetCameraArm) (* (/ (Class|PhysicsApplicablePlanetBase|GetRadiusMeters) (Math|Float|Absolute(Float) (Math|Trig|Tan(Degrees) (Variables|/Script/Engine.CameraComponent|GetFieldOfView (Variables|Default|GetCamera))))) 1e+01)))
      (Variables|Default|SetInitSpringLength _output_get)
      ;[1 1 1] causes an array index error for some reason
      (Class|PrimitiveComponent|SetMassOverrideinKg (Variables|Default|GetSphereMesh) "None" (* (Math|Float|Power 1e+01 24.0) (.Mass (Utilities|Struct|BreakLoadedValuesStruct Data))) true)
      (Variables|/Script/Engine.SpringArmComponent|SetTargetArmLength (Variables|Default|GetForceDirectionArm) (* (Class|PhysicsApplicablePlanetBase|GetRadiusMeters) 1.5))
      (Transformation|SetRelativeRotation (Variables|Default|GetSphereMesh) (Math|Rotator|MakeRotator (.Tilt (Utilities|Struct|BreakLoadedValuesStruct Data)) (.Tilt (Utilities|Struct|BreakLoadedValuesStruct Data)) 0.0) false false)
      (CallFunction|InitBinds)
      (return))))

(fn AddSplineMeshes
  ;[1 1 1] adds a cylinder mesh I made in blender (it has slices to allow bending) and bends it to make a circle for the path of the planet/moon
)

(fn InitialVel
  (bind _parentbody (Variables|Default|GetParentBody))
  (bind _data (Variables|/Script/Astrodynamics_Actual.physics_applicable_planet_base|GetData _parentbody))
  (bind (_name _bodytype _surfacetexture _mass) (Utilities|Struct|BreakLoadedValuesStruct _data))
  ;[1 1 1] for some reason Earth at 1AU has an orbital velocity of 941 km/s and a period of 0.11 days, we've done the math by hand and it should be 40 km/s, figure this shit out quickly
  (Development|PrintText _name true true "(R=1.000000,G=0.000000,B=0.016899,A=1.000000)" 4.0)
  (bind _output_get (Variables|Astrophysics|SetRelativeStartVel (Class|PhysicsApplicablePlanetBase|OrbitInitialForce (Transformation|GetDistanceTo self (Variables|Default|GetParentBody)) (Class|SplineComponent|GetTangentatSplineInputKey (Utilities|SIMOrbitPath) (Class|SplineComponent|FindInputKeyClosesttoWorldLocation (Utilities|SIMOrbitPath) (Transformation|GetWorldLocation (Variables|Default|GetSphereMesh))) "World") _mass)))
  (Development|PrintString (Utilities|String|ToString(Float) (Math|Vector|VectorLength _output_get)) true true "(R=1.000000,G=0.035352,B=0.000000,A=1.000000)" 4.0 "")
  (return (Variables|Astrophysics|GetRelativeStartVel)))

(fn CurrentOrbitProgress
  (bind _spline (Utilities|SIMOrbitPath))
  (bind _output_get (LocalVariables|SetDistRelToStart (- (Class|SplineComponent|GetDistanceAlongSplineatSplineInputKey _spline (Class|SplineComponent|FindInputKeyClosesttoWorldLocation _spline (Class|PhysicsApplicablePlanetBase|GetPlanetWorldLoc))) (Class|SplineComponent|GetDistanceAlongSplineatSplineInputKey _spline (Class|SplineComponent|FindInputKeyClosesttoWorldLocation _spline (Transformation|GetActorLocation))))))
  (if (< _output_get 0.0)
    (return (Utilities|Operators|Divide (+ (LocalVariables|GetDistRelToStart) (Spline|GetSplineLength (Utilities|SIMOrbitPath))) (Variables|Astrophysics|GetOrbitVelocity%20in%20m/s) 8.64e+04))
    (else
      (return (Utilities|Operators|Divide (LocalVariables|GetDistRelToStart) (Variables|Astrophysics|GetOrbitVelocity%20in%20m/s) 8.64e+04)))))

(fn MISNGetParent
  (return 0))

(fn MISNPlanetRadius
  (return (Class|PhysicsApplicablePlanetBase|GetRadiusMeters)))

(fn SIMGetOrbitLoc
  (return (Transformation|GetWorldLocation (Variables|Default|GetSphereMesh))))

(fn SIMOrbitCamera
  (params (Enabled? :type Boolean))
  (if Enabled?
    (Utilities|Time|SetTimerbyFunctionName 0 "RotateCam" (* 0.01 (Class|GameplayStatics|GetGlobalTimeDilation)) true)
    (else
      (Utilities|Time|ClearTimerbyFunctionName 0 "RotateCam")))
  (return))

(fn SIMSetActorDoTick
  (params (InDoTick :type Boolean))
  (return))

(fn SIMSetActorTickRate
  (params (NewTickRate :type Float%20%28double-precision%29))
  (Variables|Default|Settick NewTickRate)
  (return))