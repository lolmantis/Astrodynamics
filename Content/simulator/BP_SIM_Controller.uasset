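; Player controller for the space simulator that loads saved missions, planetary systems and spacecraft and handles view, input and UI.
; Mission loading spawns planets with spline orbit paths, then craft with data-table component masses and a rocket-equation delta-V budget.
; It switches view targets between bodies, forwards mouse camera input through an interface, feeds details to MainUI and broadcasts tick-rate changes.
; A Hohmann transfer test and temporary debug code remain.
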(event Custom|Demo%20Called
  (Development|PrintString "Request sent")
  (Default|CallBroadcastBeginPlay))

(event Custom|NewDataShow
  (params (bIsPlanet :type Boolean) (index :type Integer))
  (bind _defaultstar (Variables|Default|GetDefaultStar))
  (bind _mainui (Variables|Default|GetMainUI))
  (bind _crafts (Variables|Default|GetCrafts))
  (bind _planets (Variables|Default|GetPlanets))
  (bind _output (Utilities|Array|Get(acopy) _crafts index))
  (bind _output_2 (Utilities|Array|Get(acopy) _planets index))
  (bind _data (Variables|/Script/Astrodynamics_Actual.physics_applicable_planet_base|GetData _defaultstar))
  (bind (_name _bodytype _surfacetexture _mass _erelmass _radius) (Utilities|Struct|BreakLoadedValuesStruct _data))
  (bind _data_2 (Variables|/Script/Astrodynamics_Actual.physics_applicable_planet_base|GetData _output_2))
  (bind (_name_2 _bodytype_2 _surfacetexture_2 _mass_2 _erelmass_2 _radius_2) (Utilities|Struct|BreakLoadedValuesStruct _data_2))
  ;[1 1 1] detail gatherer with sun exception
  (if bIsPlanet
    (if (== index -1)
      (Default|GetDetails (Variables|Default|GetMainUI) _name true _bodytype (Utilities|Text|ToText(Float) _mass "HalfToEven") "N/A" (Utilities|Text|ToText(Integer) _radius) "N/A" "N/A")
      (else
        (Default|GetDetails _mainui _name_2 true _bodytype_2 (Utilities|Text|ToText(Float) _mass_2 "HalfToEven") (Utilities|Text|ToText(Float) (Math|Vector|VectorLength (Transformation|GetVelocity _output_2)) "HalfToEven") (Utilities|Text|ToText(Integer) _radius_2) "WIP" "WIP")))
    (else
      (Default|GetDetails _mainui (Utilities|Text|ToText(String) (Variables|/Script/Astrodynamics_Actual.Spacecraft|GetName _output)) false (Utilities|Text|ToText(Name) (Variables|/Script/Astrodynamics_Actual.Spacecraft|Gethull _output)) (Utilities|Text|ToText(Float) (Variables|/Script/Astrodynamics_Actual.Spacecraft|GetWetMass _output) "HalfToEven") (Utilities|Text|ToText(Float) (Math|Vector|VectorLength (Variables|/Game/simulator/BP_SIM_Craft_inheritor.BP_SIM_Craft_inheritor_C|GetVelocity _output)) "HalfToEven") (Utilities|Text|ToText(Float) (Variables|/Script/Astrodynamics_Actual.Spacecraft|GetDeltaVBudget _output) "HalfToEven") "WIP" "WIP"))))

(event EventBeginPlay
  (bind _foundwidgets (Widget|GetAllWidgetsOfClass "/Game/GlobalData/WBP_MAIN_PauseMenu.WBP_MAIN_PauseMenu_C" true))
  (if (== (Utilities|Array|Length _foundwidgets) 0)
    (bind _returnvalue (UserInterface|CreateWidget "/Game/GlobalData/WBP_MAIN_PauseMenu.WBP_MAIN_PauseMenu_C"))
    (bind _output_get (Variables|Default|SetPauseMenuQuickAccess _returnvalue))
    (UserInterface|Viewport|AddtoViewport _output_get 0)
    (Widget|SetVisibility _output_get "Hidden")))

(event EventTick
  (params (DeltaSeconds :type Float%20%28single-precision%29)))

(event EventChangeView
  (params (bPlanet :type Boolean) (index :type Integer))
  (bind _planets (Variables|Default|GetPlanets))
  (bind _crafts (Variables|Default|GetCrafts))
  (bind _output (Utilities|Array|Get(acopy) _crafts index))
  (bind _output_2 (Utilities|Array|Get(acopy) _planets index))
  (bind _returnvalue (select bPlanet _output_2 _output))
  (if (!= index -1)
    (Game|Player|SetViewTargetwithBlend _returnvalue (Math|Float|Lerp (Transformation|GetDistanceTo _returnvalue (Pawn|GetViewTarget)) 3.0 1.0) "VTBlend_EaseIn" 4.0 false)
    (else
      (Game|Player|SetViewTargetwithBlend (Variables|Default|GetDefaultStar) 0.0 "VTBlend_PreBlended" 0.0 false))))

(event EventSIMDestroySpacecraft
  (params (ActorObjectRef :type Actor%20Object%20Reference) (Index :type Integer))
  (Utilities|Array|RemoveIndex (Variables|Default|GetCrafts) Index))

(event Input|KeyboardEvents|Y
  (params (Key :type Key%20Structure :default "None"))
  ;[1 1 1] temporary solution to a weird problem
  (:Pressed
    (Development|ExecuteConsoleCommand "show splines" 0)))

(event Input|KeyboardEvents|Q
  (params (Key :type Key%20Structure :default "None"))
  ;[1 1 1] Pause Menu Displayer
  (:Pressed
    (bind _isa (Utilities|FlowControl|FlipFlop)
      (:A
        _)
      (:B
        _))
    (Widget|SetVisibility (Variables|Default|GetPauseMenuQuickAccess) (select _isa "Visible" "Hidden"))
    (Widget|SetVisibility (Variables|Default|GetMainUI) (select _isa "Hidden" "Visible"))))

(event Input|MouseEvents|MouseWheelAxis
  (params (AxisValue :type Float%20%28single-precision%29))
  (bind _returnvalue (Pawn|GetViewTarget))
  (if (Utilities|DoesObjectImplementInterface _returnvalue "/Game/simulator/Interfaces/BI_SIM_PlanetCraftInterface.BI_SIM_PlanetCraftInterface_C")
    (Class|BISIMPlanetCraftInterface|SIMScrollWheel(Message) _returnvalue AxisValue)))

(event Input|MouseEvents|RightMouseButton
  (params (Key :type Key%20Structure))
  (bind _returnvalue (Pawn|GetViewTarget))
  (bind _returnvalue_2 (Utilities|DoesObjectImplementInterface _returnvalue "/Game/simulator/Interfaces/BI_SIM_PlanetCraftInterface.BI_SIM_PlanetCraftInterface_C"))
  (:Pressed
    (if _returnvalue_2
      (Class|BISIMPlanetCraftInterface|SIMOrbitCamera(Message) _returnvalue true)))
  (:Released
    (if _returnvalue_2
      (Class|BISIMPlanetCraftInterface|SIMOrbitCamera(Message) _returnvalue false))))

(event Input|MouseEvents|LeftMouseButton
  (params (Key :type Key%20Structure))
  (:Pressed
    (if (not (Widget|IsHovered (Variables|Default|GetMainUI)))
      (Default|SIMHideMenus (Variables|Default|GetMainUI)))))

(fn ConstructionScript)

(fn LoadSystemFunction
  (params (SlotName :type String))
  ;[0.1072 1 0.8903] Empties system and begins process
  (Utilities|Array|Clear (Variables|Default|GetPlanets))
  ;[0.1684 0.8296 1] Loads Savegame and sets up basic spawn
  (bind _returnvalue (SaveGame|LoadGamefromSlot SlotName))
  (bind _asbp_syst_saved_systems (Utilities|Casting|CastToBP_SYST_Saved_systems _returnvalue))
  (for _array_element (Variables|/Game/system_creator/saving_logic/BP_SYST_Saved_systems.BP_SYST_Saved_systems_C|Getplanet_saved _asbp_syst_saved_systems)
    (bind _output_get (Variables|Loading|SetPlanetData (Utilities|Struct|MakeLoadedValuesStruct (.Name (Utilities|Struct|BreakF_SYST_planet_physics_addition _array_element)) (.body_type (Utilities|Struct|BreakF_SYST_planet_physics_addition _array_element)) (.material (Utilities|Struct|BreakF_SYST_planet_physics_addition _array_element)) (.mass (Utilities|Struct|BreakF_SYST_planet_physics_addition _array_element)) (.e_rel_mass (Utilities|Struct|BreakF_SYST_planet_physics_addition _array_element)) (.radius (Utilities|Struct|BreakF_SYST_planet_physics_addition _array_element)) (.e_rel_radius (Utilities|Struct|BreakF_SYST_planet_physics_addition _array_element)) (.worldspace_position (Utilities|Struct|BreakF_SYST_planet_physics_addition _array_element)) (.splinemap (Utilities|Struct|BreakF_SYST_planet_physics_addition _array_element)) (.Central_body (Utilities|Struct|BreakF_SYST_planet_physics_addition _array_element)) (.IsMoon (Utilities|Struct|BreakF_SYST_planet_physics_addition _array_element)))))
    (LocalVariables|SetSurfaceTemp (.surfacetexture _output_get))
    (bind _returnvalue_2 (Game|SpawnActorfromClass "/Game/simulator/BP_sim_planet.BP_sim_planet_C" (Math|Transform|MakeTransform (* (.worldpos _output_get) 1e+03) "0, 0, 0" "1.000000,1.000000,1.000000") "AlwaysSpawn" "MultiplyWithRoot" 0 0))
    ;[0.1253 1 0] used to use tags, now cleared
    (LocalVariables|SetLoadedPlanet _returnvalue_2)
    ;[0.1101 0.4313 1] Messy inbetweeny sets up actor // now all adjusted to be handled by a single function within BP_sim_planet - messy_setup_neatened
    (Utilities|Array|Add (Variables|Default|GetPhysicsPlanets) (LocalVariables|GetLoadedPlanet))
    (bind _returnvalue_3 (Utilities|Array|Add (Variables|Default|GetPlanets) (LocalVariables|GetLoadedPlanet)))
    (Class|BISIMUIConnector|AddCraft/Planet(Message) (Variables|Default|GetMainUI) true (.Name (Utilities|Struct|BreakLoadedValuesStruct (Variables|Loading|GetPlanetData))) _returnvalue_3)
    (Default|MessySetupNeatened (LocalVariables|GetLoadedPlanet) (Variables|Loading|GetPlanetData) (Variables|Default|GetDefaultStar) (Variables|Default|GetPlanets) (LocalVariables|GetSurfaceTemp) self)
    ;[0.1786 0.09567 1] Adds spline pathing for orbits and sets up spring arm length
    (for _array_element_2 (.SplineMap (Utilities|Struct|BreakLoadedValuesStruct (Variables|Loading|GetPlanetData)))
      ;;[1 0.1146 0.2444] quick for loop to set all spline points for orbit
      (Spline|AddSplinePoint (Variables|/Script/Astrodynamics_Actual.physics_applicable_planet_base|GetOrbitPath (LocalVariables|GetLoadedPlanet)) (Math|Transform|TransformLocation (Transformation|GetActorTransform (Variables|/Game/simulator/BP_sim_planet.BP_sim_planet_C|GetParentBody (LocalVariables|GetLoadedPlanet))) (* 1e+03 (Math|Transform|InverseTransformLocation (Math|Transform|MakeTransform (.WorldPos (Utilities|Struct|BreakLoadedValuesStruct (Variables|Loading|GetPlanetData)))) _array_element_2))) "Local" true)))
  (Development|PrintString "Hello")
  (for _array_element_3 (Variables|Default|GetPlanets)
    (Development|PrintText (.Name (Utilities|Struct|BreakLoadedValuesStruct (Variables|/Script/Astrodynamics_Actual.physics_applicable_planet_base|GetData _array_element_3)))))
  ;[0.7026 0.1455 1] end
  (return))

(fn LoadSpacecraftFunction
  (params (SlotName :type String) (SelectedPlanetIndex :type Integer) (SpawnPos :type Vector))
  ;[1 1 1] Initial load from savegame
  (Utilities|Array|Add (LocalVariables|GetLoadedCraftSavegames) SlotName)
  (LocalVariables|SetStartPlanetIndex SelectedPlanetIndex)
  (bind _returnvalue (SaveGame|LoadGamefromSlot SlotName))
  (bind _asbp_crftsaves (Utilities|Casting|CastToBP_CRFTSaves _returnvalue))
  (bind _returnvalue_2 (Game|SpawnActorfromClass "/Game/simulator/BP_SIM_Craft_inheritor.BP_SIM_Craft_inheritor_C" (Math|Transform|MakeTransform SpawnPos "0, 0, 0" "1.000000,1.000000,1.000000") "Undefined" "MultiplyWithRoot" 0 0))
  (Actor|Tick|SetActorTickEnabled _returnvalue_2)
  (Variables|/Game/simulator/BP_SIM_Craft_inheritor.BP_SIM_Craft_inheritor_C|SetSIMController _returnvalue_2 self)
  (Default|InitialiseBindings _returnvalue_2)
  ;[1 1 1] Fancy initialiser & setting of Destroy tag for cleaning up
  (bind _output_get (Variables|Loading|SetLoadedCraft _returnvalue_2))
  (Variables|/Game/mission_creator/BP_MISN_CRFT.BP_MISN_CRFT_C|SetStartPlanetOrbit _output_get (LocalVariables|GetStartPlanetIndex))
  (bind _total_mass (CallFunction|GetTotalMass (Utilities|Array|MakeArray (.GyroStruct (Utilities|Struct|BreakF_CRFT_CMPNTSave (Variables|/Game/spacecraft_creator/SavingLogic/BP_CRFTSaves.BP_CRFTSaves_C|GetSaveStructure _asbp_crftsaves))) (.ReactStruct (Utilities|Struct|BreakF_CRFT_CMPNTSave (Variables|/Game/spacecraft_creator/SavingLogic/BP_CRFTSaves.BP_CRFTSaves_C|GetSaveStructure _asbp_crftsaves))) (.WhelStruct (Utilities|Struct|BreakF_CRFT_CMPNTSave (Variables|/Game/spacecraft_creator/SavingLogic/BP_CRFTSaves.BP_CRFTSaves_C|GetSaveStructure _asbp_crftsaves))) (.ThruStruct (Utilities|Struct|BreakF_CRFT_CMPNTSave (Variables|/Game/spacecraft_creator/SavingLogic/BP_CRFTSaves.BP_CRFTSaves_C|GetSaveStructure _asbp_crftsaves))) (.HullStruct (Utilities|Struct|BreakF_CRFT_CMPNTSave (Variables|/Game/spacecraft_creator/SavingLogic/BP_CRFTSaves.BP_CRFTSaves_C|GetSaveStructure _asbp_crftsaves))))))
  (Class|Spacecraft|Initialiser (Variables|Loading|GetLoadedCraft) (.Name (Utilities|Struct|BreakF_CRFT_CMPNTSave (Variables|/Game/spacecraft_creator/SavingLogic/BP_CRFTSaves.BP_CRFTSaves_C|GetSaveStructure _asbp_crftsaves))) (.FuelCapacity (Utilities|Struct|BreakF_CRFT_CMPNTSave (Variables|/Game/spacecraft_creator/SavingLogic/BP_CRFTSaves.BP_CRFTSaves_C|GetSaveStructure _asbp_crftsaves))) (.BatteryCapacity (Utilities|Struct|BreakF_CRFT_CMPNTSave (Variables|/Game/spacecraft_creator/SavingLogic/BP_CRFTSaves.BP_CRFTSaves_C|GetSaveStructure _asbp_crftsaves))) _total_mass (+ _total_mass (* (.FuelCapacity (Utilities|Struct|BreakF_CRFT_CMPNTSave (Variables|/Game/spacecraft_creator/SavingLogic/BP_CRFTSaves.BP_CRFTSaves_C|GetSaveStructure _asbp_crftsaves))) 1e+03)) (.Crew (Utilities|Struct|BreakF_CRFT_CMPNTSave (Variables|/Game/spacecraft_creator/SavingLogic/BP_CRFTSaves.BP_CRFTSaves_C|GetSaveStructure _asbp_crftsaves))) (.HullStruct (Utilities|Struct|BreakF_CRFT_CMPNTSave (Variables|/Game/spacecraft_creator/SavingLogic/BP_CRFTSaves.BP_CRFTSaves_C|GetSaveStructure _asbp_crftsaves))) (Utilities|Array|MakeArray (.ThruStruct (Utilities|Struct|BreakF_CRFT_CMPNTSave (Variables|/Game/spacecraft_creator/SavingLogic/BP_CRFTSaves.BP_CRFTSaves_C|GetSaveStructure _asbp_crftsaves)))) (Utilities|Array|MakeArray (.ReactStruct (Utilities|Struct|BreakF_CRFT_CMPNTSave (Variables|/Game/spacecraft_creator/SavingLogic/BP_CRFTSaves.BP_CRFTSaves_C|GetSaveStructure _asbp_crftsaves)))) (Utilities|Array|MakeArray (.WhelStruct (Utilities|Struct|BreakF_CRFT_CMPNTSave (Variables|/Game/spacecraft_creator/SavingLogic/BP_CRFTSaves.BP_CRFTSaves_C|GetSaveStructure _asbp_crftsaves)))) (Utilities|Array|MakeArray (.GyroStruct (Utilities|Struct|BreakF_CRFT_CMPNTSave (Variables|/Game/spacecraft_creator/SavingLogic/BP_CRFTSaves.BP_CRFTSaves_C|GetSaveStructure _asbp_crftsaves)))))
  ;[1 1 1] First time run for Delta-V budget
  (bind _returnvalue_3 (Utilities|GetDataTableRow "/Game/spacecraft_creator/components/DataTables/DT_Thrusters.DT_Thrusters" (Utilities|Array|Get(acopy) (Variables|/Script/Astrodynamics_Actual.Spacecraft|Getthrusters (Variables|Loading|GetLoadedCraft))))
    (:then
      (bind _velocity (Class|Spacecraft|RocketEquation (Variables|Loading|GetLoadedCraft) (.SpecificImpulse (Utilities|Struct|BreakF_CRFT_Thrusters _returnvalue_3)) (Variables|/Script/Astrodynamics_Actual.Spacecraft|GetWetMass (Variables|Loading|GetLoadedCraft)) (Variables|/Script/Astrodynamics_Actual.Spacecraft|GetDryMass (Variables|Loading|GetLoadedCraft))))
      (Variables|/Script/Astrodynamics_Actual.Spacecraft|SetDeltaVBudget (Variables|Loading|GetLoadedCraft) _velocity)
      (Default|UpdateMesh (Variables|Loading|GetLoadedCraft))
      (bind _returnvalue_4 (Utilities|Array|Add (Variables|Default|GetCrafts) (Variables|Loading|GetLoadedCraft)))
      (Utilities|FlowControl|Sequence
        (:then_0
          (Class|BISIMUIConnector|AddCraft/Planet(Message) (Variables|Default|GetMainUI) false (Utilities|Text|FormatText "{str}" (Variables|/Script/Astrodynamics_Actual.Spacecraft|GetName (Variables|Loading|GetLoadedCraft))) _returnvalue_4))
        (:then_1
          ;[1 1 1] Quick test of the Hohmann transfer function
          (bind _returnvalue_5 (Utilities|GetDataTableRow "/Game/planet_creator/DT_PlanetData.DT_PlanetData" "Earth")
            (:then
              (bind (_trnsfrsemimjraxis _trnsfrsemiminraxis _periapsisvel _apoapsisvel _firstdeltav _finaldeltav _totaldeltav) (Class|Spacecraft|Hohmann (Variables|Loading|GetLoadedCraft) (Class|KismetSystemLibrary|MakeLiteralInteger 7000) (Class|KismetSystemLibrary|MakeLiteralInteger 20000) (.Planet_mass (Utilities|Struct|BreakF_PLNT_Data _returnvalue_5)) (Math|Float|MakeLiteralFloat 0.0)))
              (for _array_element (Utilities|Array|MakeArray _trnsfrsemimjraxis _trnsfrsemiminraxis _periapsisvel _apoapsisvel _firstdeltav _finaldeltav _totaldeltav)
                (Development|PrintString (Utilities|String|ToString(Float) _array_element)))
              (return (Variables|Loading|GetLoadedCraft)))))))))

(fn LoadMissionFunction
  (params (SlotName :type String))
  (bind _returnvalue (SaveGame|LoadGamefromSlot SlotName))
  (Variables|Default|Setsystem%20tick%20rate 0.0)
  (bind _asbp_misn_save_object (Utilities|Casting|CastToBP_MISN_Save_Object _returnvalue))
  (CallFunction|LoadSystemFunction (Variables|/Game/mission_creator/Saving/BP_MISN_Save_Object.BP_MISN_Save_Object_C|GetSystemSavegame _asbp_misn_save_object))
  (for _array_element (Variables|/Game/mission_creator/Saving/BP_MISN_Save_Object.BP_MISN_Save_Object_C|GetSpacecraft _asbp_misn_save_object)
    (bind _loadedcrft (CallFunction|LoadSpacecraftFunction (.CraftSave (Utilities|Struct|BreakF_MISN_Craft_With_Struct_Pairs _array_element)) (.StartPlanetIndex (Utilities|Struct|BreakF_MISN_Craft_With_Struct_Pairs _array_element)) (.CraftPosition (Utilities|Struct|BreakF_MISN_Craft_With_Struct_Pairs _array_element))))
    (Variables|Loading|SetLoadedCraft _loadedcrft)
    (Utilities|FlowControl|Sequence
      (:then_0
        (for _array_element_2 (.InitialOrbitSplinePoints (Utilities|Struct|BreakF_MISN_Craft_With_Struct_Pairs _array_element))
          (Spline|AddSplinePoint (Variables|/Game/simulator/BP_sim_planet.BP_sim_planet_C|GetSpacecraftDraw (Utilities|Array|Get(acopy) (Variables|Default|GetPlanets) (.StartPlanetIndex (Utilities|Struct|BreakF_MISN_Craft_With_Struct_Pairs _array_element)))) (+ _array_element_2 (- (Transformation|GetActorLocation (Variables|Loading|GetLoadedCraft)) (Transformation|GetWorldLocation (Variables|/Script/Astrodynamics_Actual.physics_applicable_planet_base|GetSphereMesh (Utilities|Array|Get(acopy) (Variables|Default|GetPlanets) (.StartPlanetIndex (Utilities|Struct|BreakF_MISN_Craft_With_Struct_Pairs _array_element))))))) "Local" true)))
      (:then_1
        (Variables|/Game/mission_creator/BP_MISN_CRFT.BP_MISN_CRFT_C|SetMovementSequence (Variables|Loading|GetLoadedCraft) (.F_MISN_CraftMoves (Utilities|Struct|BreakF_MISN_Craft_With_Struct_Pairs _array_element))))))
  (Game|Player|SetViewTargetwithBlend (Variables|Loading|GetLoadedCraft) 0.0 "VTBlend_Linear" 0.0 false)
  (return))

(fn GetTotalMas
  (params (Comp%20Names :type Array%20of%20Names))
  (return 0.0))

(fn GetComponentMass
  (params (InName :type Name))
  (switch string (Utilities|String|Left (Utilities|String|ToString(Name) InName) 4)
    (:HUL_
      (bind _returnvalue (Utilities|GetDataTableRow "/Game/spacecraft_creator/components/DataTables/DT_Hulls.DT_Hulls" InName)
        (:then
          (return (.Mass (Utilities|Struct|BreakF_CRFT_Hulls _returnvalue))))))
    (:GYR_
      (bind _returnvalue_2 (Utilities|GetDataTableRow "/Game/spacecraft_creator/components/DataTables/DT_Gyroscopes.DT_Gyroscopes" InName)
        (:then
          (return (.Mass (Utilities|Struct|BreakF_CRFT_Gyroscopes _returnvalue_2))))))
    (:WHL_
      (bind _returnvalue_3 (Utilities|GetDataTableRow "/Game/spacecraft_creator/components/DataTables/DT_ReactWheels.DT_ReactWheels" InName)
        (:then
          (return (.Mass (Utilities|Struct|BreakF_CRFT_ReactWheels _returnvalue_3))))))
    (:ION_
      (bind _returnvalue_4 (Utilities|GetDataTableRow "/Game/spacecraft_creator/components/DataTables/DT_Thrusters.DT_Thrusters" InName)
        (:then
          (return (.Mass (Utilities|Struct|BreakF_CRFT_Thrusters _returnvalue_4))))))
    (:RCT_
      (bind _returnvalue_5 (Utilities|GetDataTableRow "/Game/spacecraft_creator/components/DataTables/DT_Reactors.DT_Reactors" InName)
        (:then
          (return (.Mass (Utilities|Struct|BreakF_CRFT_Reactors _returnvalue_5))))))))

(fn GetTotalMass
  (params (Comp%20Names :type Array%20of%20Names))
  (for _array_element Comp%20Names
    (bind _mass (CallFunction|GetComponentMass _array_element))
    (LocalVariables|SetMass (+ _mass (LocalVariables|GetMass))))
  (return (LocalVariables|GetMass)))

(fn SIMGetOrbitLoc
  (return "0, 0, 0"))

(fn SIMSetActorDoTick
  (params (InDoTick :type Boolean))
  (return))

(fn SIMSetActorTickRate
  (params (NewTickRate :type Float%20%28double-precision%29))
  (Variables|Default|Setsystem%20tick%20rate NewTickRate)
  (Default|CallBroadcastTickRate)
  (return))